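; Usable ammo item that loads itself into the character's equipped two-handed ranged weapon.
; On use, it checks the equipment inventory's dual-hand slot for that weapon archetype, then passes its own template ID to SetAmmo through the projectile weapon interface.
; It always reports itself as usable, even though use does nothing without a matching weapon, and it refuses items dropped onto it.
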(event `self.OnUseItem`
  (params (invokingCharacter :type "ConanCharacter Object Reference"))
  (if (`ConanCharacter.HasWeaponsEquipped` invokingCharacter)
    (bind _returnvalue (`ConanCharacter.GetEquipmentInventoryNative` invokingCharacter))
    (bind _returnvalue_2 (`EquipmentInventory.GetItemAtSlot` _returnvalue "DualHand"))
    (if (`KismetSystemLibrary.IsValid` _returnvalue_2)
      (if (`|EnumEquality` (`GameItem.WeaponArcheType` _returnvalue_2) "TwoHanded_Ranged")
        (bind _asbp_projectile_weapon_interface (cast `/Game/Items/BP_ProjectileWeaponInterface` _returnvalue_2))
        (`/Game/Items/BP_ProjectileWeaponInterface.SetAmmo` _asbp_projectile_weapon_interface (`self.TemplateID`))))))

(fn `CanItemBeDroppedOnItem`
  (params (droppedItem :type "GameItem Object Reference") (srcInventory :type "ItemInventory Object Reference") (srcIndex :type Integer))
  (returns (ReturnValue :type Boolean))
  (return false))

(fn `CanUseItem`
  (params (invokingCharacter :type "ConanCharacter Object Reference"))
  (returns (ReturnValue :type Boolean))
  (return true))