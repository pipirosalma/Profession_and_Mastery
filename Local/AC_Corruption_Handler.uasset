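; Player character component that changes the character's appearance as Corruption energy builds.
; Tick steps the effect up through three energy thresholds and resets it once energy falls below a lower threshold.
; ChangeLook forwards to ChangeLook_SRV, which rebuilds the character layout, altering eye tint, then hair and eyebrows, then skin.
; SetDefaults caches original tints, but reset, also run on EndPlay, restores only skin and eyes.
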(event `self.ReceiveTick`
  (params (DeltaSeconds :type "Float (single-precision)"))
  (bind _asbase_player_char (cast `/Game/Characters/BasePlayerChar` (`self.GetOwner`)))
  (bind _returnvalue (`EnergyReceiverComponent.GetEnergy` (`/Game/Characters/BasePlayerChar.BPEnergyReceiver` _asbase_player_char) "EnergyType_Corruption"))
  (`/Game/Systems/BP_MacroGlobal.And+Branch` (!= (`self.CorruptionEffect`) 0) (> 700.0 _returnvalue)
    (:`True`
      (bind _output_get (set `self.CorruptionEffect` 0))
      (`self.ChangeLook` _output_get))
    (:`False`
      (`/Game/Systems/BP_MacroGlobal.And+Branch` (> _returnvalue 750.0) (== (`self.CorruptionEffect`) 0)
        (:`True`
          (bind _output_get_2 (set `self.CorruptionEffect` 1))
          (`self.ChangeLook` _output_get_2))
        (:`False`
          (`/Game/Systems/BP_MacroGlobal.And+Branch` (> _returnvalue 1001.0) (== (`self.CorruptionEffect`) 1)
            (:`True`
              (bind _output_get_3 (set `self.CorruptionEffect` 2))
              (`self.ChangeLook` _output_get_3))
            (:`False`
              (`/Game/Systems/BP_MacroGlobal.And+Branch` (> _returnvalue 1750.0) (== (`self.CorruptionEffect`) 2)
                (:`True`
                  (bind _output_get_4 (set `self.CorruptionEffect` 3))
                  (`self.ChangeLook` _output_get_4))))))))))

(event `self.ReceiveEndPlay`
  (params (EndPlayReason :type "EEndPlayReason Enum" :default "Destroyed"))
  (`self.ChangeLook` 0))

(event `ChangeLook`
  (params (CorruptionEffectLVL :type Integer))
  (`self.ChangeLook_SRV` CorruptionEffectLVL))

(event `ChangeLook_SRV`
  (params (CorruptionEffectLVL :type Integer))
  (`self.SetDefaults`)
  (bind _asbase_player_char (cast `/Game/Characters/BasePlayerChar` (`self.GetOwner`)))
  (switch `int` CorruptionEffectLVL
    (:`Default`
      (bind (_meshlayout _texturelayout _tintlayout _boolparams _intparams _scalarparams _enumparams _armourdyeparams) (break `CharacterLayout` (`/Game/Characters/BasePlayerChar.CharacterLayout` _asbase_player_char)))
      (bind (_skin _hair _facialhair _eyes _eyebrows _eyemakeup _lipmakeup _warpaint) (break `CharacterTintLayout` _tintlayout))
      (`/Game/Characters/BasePlayerChar.SetCharacterLayout` _asbase_player_char (make `CharacterLayout` _meshlayout _texturelayout (make `CharacterTintLayout` 21 _hair _facialhair _eyes _eyebrows _eyemakeup _lipmakeup _warpaint) _boolparams _intparams _scalarparams _enumparams _armourdyeparams) :!label _label))
    (:`0`
      (bind (_meshlayout_2 _texturelayout_2 _tintlayout_2 _boolparams_2 _intparams_2 _scalarparams_2 _enumparams_2 _armourdyeparams_2) (break `CharacterLayout` (`/Game/Characters/BasePlayerChar.CharacterLayout` _asbase_player_char)))
      (bind (_skin_2 _hair_2 _facialhair_2 _eyes_2 _eyebrows_2 _eyemakeup_2 _lipmakeup_2 _warpaint_2) (break `CharacterTintLayout` _tintlayout_2))
      (`/Game/Characters/BasePlayerChar.SetCharacterLayout` _asbase_player_char (make `CharacterLayout` _meshlayout_2 _texturelayout_2 (make `CharacterTintLayout` (`self.Skin`) _hair_2 _facialhair_2 (`self.Eyes`) _eyebrows_2 _eyemakeup_2 _lipmakeup_2 _warpaint_2) _boolparams_2 _intparams_2 _scalarparams_2 _enumparams_2 _armourdyeparams_2)))
    (:`1`
      (bind (_meshlayout_3 _texturelayout_3 _tintlayout_3 _boolparams_3 _intparams_3 _scalarparams_3 _enumparams_3 _armourdyeparams_3) (break `CharacterLayout` (`/Game/Characters/BasePlayerChar.CharacterLayout` _asbase_player_char)))
      (bind (_skin_3 _hair_3 _facialhair_3 _eyes_3 _eyebrows_3 _eyemakeup_3 _lipmakeup_3 _warpaint_3) (break `CharacterTintLayout` _tintlayout_3))
      (`/Game/Characters/BasePlayerChar.SetCharacterLayout` _asbase_player_char (make `CharacterLayout` _meshlayout_3 _texturelayout_3 (make `CharacterTintLayout` _skin_3 _hair_3 _facialhair_3 20 _eyebrows_3 _eyemakeup_3 _lipmakeup_3 _warpaint_3) _boolparams_3 _intparams_3 _scalarparams_3 _enumparams_3 _armourdyeparams_3)))
    (:`2`
      (bind (_meshlayout_4 _texturelayout_4 _tintlayout_4 _boolparams_4 _intparams_4 _scalarparams_4 _enumparams_4 _armourdyeparams_4) (break `CharacterLayout` (`/Game/Characters/BasePlayerChar.CharacterLayout` _asbase_player_char)))
      (bind (_skin_4 _hair_4 _facialhair_4 _eyes_4 _eyebrows_4 _eyemakeup_4 _lipmakeup_4 _warpaint_4) (break `CharacterTintLayout` _tintlayout_4))
      (`/Game/Characters/BasePlayerChar.SetCharacterLayout` _asbase_player_char (make `CharacterLayout` _meshlayout_4 _texturelayout_4 (make `CharacterTintLayout` _skin_4 0 _facialhair_4 _eyes_4 0 _eyemakeup_4 _lipmakeup_4 _warpaint_4) _boolparams_4 _intparams_4 _scalarparams_4 _enumparams_4 _armourdyeparams_4)))
    (:`3`
      (goto _label))))