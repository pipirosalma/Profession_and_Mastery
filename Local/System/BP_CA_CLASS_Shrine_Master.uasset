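; Master class shrine for a Conan Exiles mod that lets an interacting player permanently pick the class it offers.
; On client activation it looks up the class description in a data table and shows it, provided the player's class matches the offered one or a specific enum value; otherwise it shows a locked notice.
; Two chained Yes/No boxes lead to the player's main component learning the class feat and a HUD announcement.
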(event `Confirm`
  (params (result :type "EMessageBoxDialogResult Enum"))
  (bind _returnvalue (`|GetEnumeratorNameAsString` (`self.OfferedClass`)))
  (if (`|EnumEquality` result "Yes")
    (bind _returnvalue_2 (`MessageBoxWidget.CreateMessageBox` self "YesNo" (`KismetStringLibrary.Concat_StrStr` "Class: " _returnvalue) (`KismetStringLibrary.Concat_StrStr` "Are you sure You want your class to be a(n)" _returnvalue "?\n" "YOU CAN'T CHANGE ONCE YOU PICK A CLASS ")))
    (`MessageBoxWidget.ShowMessageBox` _returnvalue_2)
    (add `MessageBoxWidget.SignalUserActionPerformed` _returnvalue_2 (delegate `MessageBoxResult`))))

(event `InteractableInterface.ClientInteractableActivate`
  (params (Component :type "PrimitiveComponent Object Reference") (Instigator :type "PlayerController Object Reference") (HitIndex :type Integer))
  (bind _asbase_player_char (cast `/Game/Characters/BasePlayerChar` (cast `ConanCharacter` (`Controller.K2_GetPawn` Instigator) :!pure true)))
  (`self.GetDescription`
    (:`Completed`
      (bind _playerclass (`/Game/Mods/Profession_and_Mastery/AC_Actor_Component_Main.PlayerClass` (`self.GetComponentByClass` _asbase_player_char "/Game/Mods/Profession_and_Mastery/AC_Actor_Component_Main.AC_Actor_Component_Main_C")))
      (if (or (`|EnumEquality` _playerclass "NewEnumerator7") (`|EnumEquality` (`self.OfferedClass`) _playerclass))
        (bind _returnvalue (`MessageBoxWidget.CreateMessageBox` self "YesNo" (`KismetStringLibrary.Concat_StrStr` "Class: " (`|GetEnumeratorNameAsString` (`self.OfferedClass`))) (`KismetTextLibrary.Conv_TextToString` (`self.ClassDescription`))))
        (`MessageBoxWidget.ShowMessageBox` _returnvalue)
        (add `MessageBoxWidget.SignalUserActionPerformed` _returnvalue (delegate `Confirm`))
        (else
          (bind _returnvalue_2 (`MessageBoxWidget.CreateMessageBox` self "OK" "Class Choice Locked" (`KismetStringLibrary.Concat_StrStr` "You alread have a class:" (`|GetEnumeratorNameAsString` _playerclass))))
          (`MessageBoxWidget.ShowMessageBox` _returnvalue_2))))))

(event `MessageBoxResult`
  (params (result :type "EMessageBoxDialogResult Enum"))
  (bind _offeredclass (`self.OfferedClass`))
  (bind _returnvalue (`|GetEnumeratorNameAsString` _offeredclass))
  (if (`|EnumEquality` result "Yes")
    (bind _returnvalue_2 (`self.GetComponentByClass` (stale `InteractableInterface.ClientInteractableActivate` _asbase_player_char) "/Game/Mods/Profession_and_Mastery/AC_Actor_Component_Main.AC_Actor_Component_Main_C"))
    (`/Game/Mods/Profession_and_Mastery/AC_Actor_Component_Main.LearnClassFeat` _returnvalue_2 _offeredclass)
    (`ConanCharacter.ClientHUDShowFIFOEx` (`/Game/Mods/Profession_and_Mastery/AC_Actor_Component_Main.BasePlayerSelf` _returnvalue_2) "Journey" (`KismetTextLibrary.Conv_StringToText` (`KismetStringLibrary.Concat_StrStr` "Your class is now " _returnvalue)) (`KismetTextLibrary.Conv_StringToText` _returnvalue))))

(fn `UserConstructionScript`
  (`parent.UserConstructionScript`))