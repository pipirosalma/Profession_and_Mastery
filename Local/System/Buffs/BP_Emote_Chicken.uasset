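; BP_Emote_Chicken is a buff that shifts the affected character's NaturalArmor stat for as long as it is active.
; StartBuff scales the amount by buff potency, positive when the owner's controller is the instigator and negative otherwise, then calls the parent.
; The start and cleared effect events add and then reverse that modifier.
; GetEffectDescription returns fixed encumbrance text, which does not match the armor effect.
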(event `self.StartBuff`
  (params (BuffPotency :type Integer) (DamageCauser :type "Actor Object Reference") (OwningCharacter :type "ConanCharacter Object Reference") (Instigator :type "Controller Object Reference"))
  (bind _returnvalue (* BuffPotency 40))
  (if (== (`Pawn.GetController` OwningCharacter) Instigator)
    (set `self.ArmorValue` _returnvalue)
    (else
      (set `self.ArmorValue` (* _returnvalue -1))))
  (`parent.StartBuff` BuffPotency DamageCauser OwningCharacter Instigator))

(event `self.GameplayEffectToApplyOnBuffStart`
  (`ConanCharacter.AddFloatStatModifier` (`self.OwningCharacter`) "NaturalArmor" "Default" "Add" (`KismetMathLibrary.Conv_IntToDouble` (`self.ArmorValue`)) "Replace"))

(event `self.GameplayEffectToApplyOnBuffCleared`
  (`ConanCharacter.AddFloatStatModifier` (`self.OwningCharacter`) "NaturalArmor" "Default" "Add" (`KismetMathLibrary.Conv_IntToDouble` (* (`self.ArmorValue`) -1)) "Replace"))

(fn `GetEffectDescription`
  (returns (Description :type Text))
  (return (`|FormatText` "Encumberance increased by 3")))