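; Base buff Blueprint for drugs, which applies a screen effect and a stamina regen change to the owning character.
; On start, it sets a custom post-process effect from BuffType via the player's main actor component, then adds BuffStaminaRegen to the combat character's regen modifier.
; On clear, it resets the effect and subtracts the same amount.
; Both stamina changes only run if the player character cast succeeds.
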(event `self.StartBuff`
  (params (BuffPotency :type Integer) (DamageCauser :type "Actor Object Reference") (OwningCharacter :type "ConanCharacter Object Reference") (Instigator :type "Controller Object Reference"))
  (`parent.StartBuff` BuffPotency DamageCauser OwningCharacter Instigator))

(event `self.GameplayEffectToApplyOnBuffStart`
  (bind _asbase_player_char (cast `/Game/Characters/BasePlayerChar` (`self.OwningCharacter`)))
  (`/Game/Mods/Profession_and_Mastery/AC_Actor_Component_Main.CustomPPEffect` (`Actor.GetComponentByClass` _asbase_player_char "/Game/Mods/Profession_and_Mastery/AC_Actor_Component_Main.AC_Actor_Component_Main_C") (`self.BuffType`))
  (bind _asbase_bpcombat (cast `/Game/Characters/BaseBPCombat` (`self.OwningCharacter`)))
  (`/Game/Characters/BaseBPCombat.AdjustStaminaRegenMod` _asbase_bpcombat (`self.BuffStaminaRegen`)))

(event `self.GameplayEffectToApplyOnBuffCleared`
  (bind _asbase_player_char (cast `/Game/Characters/BasePlayerChar` (`self.OwningCharacter`)))
  (`/Game/Mods/Profession_and_Mastery/AC_Actor_Component_Main.CustomPPEffect` (`Actor.GetComponentByClass` _asbase_player_char "/Game/Mods/Profession_and_Mastery/AC_Actor_Component_Main.AC_Actor_Component_Main_C") 0)
  (bind _asbase_bpcombat (cast `/Game/Characters/BaseBPCombat` (`self.OwningCharacter`)))
  (`/Game/Characters/BaseBPCombat.AdjustStaminaRegenMod` _asbase_bpcombat (* (`self.BuffStaminaRegen`) -1.0)))