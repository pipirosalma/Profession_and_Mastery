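; BP_Warcry_Brawler is a buff, named as the Brawler warcry, that raises the owning character's Might attribute while active.
; On buff start it adds twice the buff potency to Might as a merged integer stat modifier.
; When cleared it adds the negated amount to undo the bonus, after calling the parent buff logic in each case.
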(event `self.ReceiveBeginPlay`)

(event `self.StartBuff`
  (params (BuffPotency :type Integer) (DamageCauser :type "Actor Object Reference") (OwningCharacter :type "ConanCharacter Object Reference") (Instigator :type "Controller Object Reference"))
  (`parent.StartBuff` BuffPotency DamageCauser OwningCharacter Instigator))

(event `self.GameplayEffectToApplyOnBuffStart`
  (`parent.GameplayEffectToApplyOnBuffStart`)
  (`ConanCharacter.AddIntStatModifier` (`self.OwningCharacter`) "AttributeMight" "Default" "Add" (* (`self.BuffPotency`) 2) "Merge"))

(event `self.GameplayEffectToApplyOnBuffCleared`
  (`parent.GameplayEffectToApplyOnBuffCleared`)
  (`ConanCharacter.AddIntStatModifier` (`self.OwningCharacter`) "AttributeMight" "Default" "Add" (* (* (`self.BuffPotency`) 2) -1) "Merge"))