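; BP_Emote_Sexy is a buff, named for an emote, that drains Corruption energy from the character that owns it.
; StartBuff only forwards to the parent implementation.
; Each Tick finds the owner's first BPEnergyReceiver, if any, and lowers its Corruption by the buff potency plus a fixed offset, clamped at zero and with no heatmap force.
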(event `self.StartBuff`
  (params (BuffPotency :type Integer) (DamageCauser :type "Actor Object Reference") (OwningCharacter :type "ConanCharacter Object Reference") (Instigator :type "Controller Object Reference"))
  (`parent.StartBuff` BuffPotency DamageCauser OwningCharacter Instigator))

(event `self.ReceiveTick`
  (params (DeltaSeconds :type "Float (single-precision)"))
  (bind _returnvalue (`Actor.K2_GetComponentsByClass` (stale `self.StartBuff` OwningCharacter) "/Game/Systems/BPEnergyReceiver.BPEnergyReceiver_C"))
  (if (> (`KismetArrayLibrary.Array_Length` _returnvalue) 0)
    (bind _item (`KismetArrayLibrary.Array_Get` _returnvalue))
    (`EnergyReceiverComponent.SetEnergy` _item "EnergyType_Corruption" (`KismetMathLibrary.FMax` (- (`EnergyReceiverComponent.GetEnergy` _item "EnergyType_Corruption") (`KismetMathLibrary.Conv_IntToDouble` (+ (`self.BuffPotency`) 2)))) 0.0)))