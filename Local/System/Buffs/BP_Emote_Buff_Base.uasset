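; Base Blueprint for emote buffs, which grant a temporary bonus to a character stat.
; On start it removes every buff in its EmoteBuffs list from the player's buff system before running the parent start logic, so emote buffs replace one another.
; It adds twice BuffPotency to BonusAttribute and subtracts the same amount when cleared.
; The effect description is fixed encumbrance text, independent of the actual stat and amount.
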(event `self.StartBuff`
  (params (BuffPotency :type Integer) (DamageCauser :type "Actor Object Reference") (OwningCharacter :type "ConanCharacter Object Reference") (Instigator :type "Controller Object Reference"))
  (`self.RemoveOtherEmoteBuffs` OwningCharacter)
  (`parent.StartBuff` BuffPotency DamageCauser OwningCharacter Instigator))

(event `self.GameplayEffectToApplyOnBuffStart`
  (`ConanCharacter.AddIntStatModifier` (`self.OwningCharacter`) (`self.BonusAttribute`) "Default" "Add" (* (`self.BuffPotency`) 2) "Merge"))

(event `self.GameplayEffectToApplyOnBuffCleared`
  (`ConanCharacter.AddIntStatModifier` (`self.OwningCharacter`) (`self.BonusAttribute`) "Default" "Add" (* (* (`self.BuffPotency`) 2) -1) "Merge"))

(fn `GetEffectDescription`
  (returns (Description :type Text))
  (return (`|FormatText` "Encumberance increased by 3")))

(fn `RemoveOtherEmoteBuffs`
  (params (Object :type "Object Object Reference"))
  (bind _asbase_player_char (cast `/Game/Characters/BasePlayerChar` Object)
    (:`then`
      (for _array_element (`self.EmoteBuffs`)
        (`/Game/Systems/Buffs/00_BP_AC_BuffSystem.RemoveBuff` (`/Game/Characters/BaseBPCombat.00_BP_AC_BuffSystem` _asbase_player_char) _array_element))
      (return))
    (:`CastFailed`
      (return))))