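; BP_Emote_Belly is a stackable buff that raises its owning character's health regeneration while active.
; The regen multiplier is buff potency times stack size times a base value, doubled if the owner has the Vitality_40 perk, and is recalculated on stack changes.
; The setter applies only the delta to BaseBPCombat and zeroes on clear.
; A RepNotify on the multiplier signals the percentage description to refresh.
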(event `self.StartBuff`
  (params (BuffPotency :type Integer) (DamageCauser :type "Actor Object Reference") (OwningCharacter :type "ConanCharacter Object Reference") (Instigator :type "Controller Object Reference"))
  (`parent.StartBuff` BuffPotency DamageCauser OwningCharacter Instigator))

(event `self.GameplayEffectToApplyOnBuffStart`
  (`self.SetCurrentHealthRegenMultiplier` (`self.CalculateHealthRegenMultiplier`)))

(event `self.GameplayEffectToApplyOnBuffCleared`
  (`self.SetCurrentHealthRegenMultiplier` 0.0))

(event `self.AdjustStackSize`
  (params (StackAdjustment :type Integer))
  (`parent.AdjustStackSize` StackAdjustment)
  (`self.SetCurrentHealthRegenMultiplier` (`self.CalculateHealthRegenMultiplier`)))

(fn `CalculateHealthRegenMultiplier`
  (returns (ReturnValue :type "Float (double-precision)"))
  (locals (PerkModifier :type "Float (double-precision)"))
  (bind _asi_perk_system_interface (cast `/Game/Systems/Perks/I_PerkSystemInterface` (`Actor.GetComponentByClass` (`self.OwningCharacter`) "/Script/ConanSandbox.PerkSystemComponent"))
    (:`then`
      (bind _hasperk (`/Game/Systems/Perks/I_PerkSystemInterface.HasPerk` _asi_perk_system_interface "Vitality_40"))
      (if _hasperk
        (set `local.PerkModifier` 2.0)
        (else
          (set `local.PerkModifier` 1.0 :!label _label))))
    (:`CastFailed`
      (goto _label)))
  (return (* (* (* (`self.BuffPotency`) (`self.StackSize`)) (`self.BuffHealthRegen`)) (`local.PerkModifier`))))

(fn `GetEffectDescription`
  (returns (Description :type Text))
  (return (`|FormatText` "Increase health regeneration by {RegenMultiplier}%." (`KismetMathLibrary.Round` (* (`self.CurrentHealthRegenMultiplier`) 100.0)))))

(fn `OnRep_CurrentHealthRegenMultiplier`
  (`self.SignalEffectDescriptionChanged` self))

(fn `SetCurrentHealthRegenMultiplier`
  (params (NewMultiplier :type "Float (double-precision)"))
  (bind _asbase_bpcombat (cast `/Game/Characters/BaseBPCombat` (`self.OwningCharacter`)))
  (`/Game/Characters/BaseBPCombat.AdjustHealthRegen` _asbase_bpcombat (- NewMultiplier (`self.CurrentHealthRegenMultiplier`)))
  (set `self.CurrentHealthRegenMultiplier` NewMultiplier))