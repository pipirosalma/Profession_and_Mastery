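; Hunter Warcry buff that raises the owning character's Accuracy in proportion to buff potency and grants a movement speed boost.
; Start and clear effects add or subtract the stat modifier and apply or remove the speed multiplier through the combat interface, which is cached in ClientStartBuff.
; Client start and clear events replay only the speed change on non-server machines, so the server does not apply it twice.
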(event `self.ReceiveBeginPlay`)

(event `self.GameplayEffectToApplyOnBuffStart`
  (`ConanCharacter.AddIntStatModifier` (`self.OwningCharacter`) "AttributeAccuracy" "Default" "Add" (* (`self.BuffPotency`) 2) "Merge")
  (`parent.GameplayEffectToApplyOnBuffStart`)
  (bind _output_get (set `self.MovementSpeedMultiplier` 1.2 :!label _label))
  (`/Game/Systems/Interfaces/IsBaseBPCombatInterface.AdjustMovementSpeedMultiplier` (`self.ConbatInterface`) true _output_get))

(event `self.ClientStartBuff`
  (params (OwningCharacter :type "ConanCharacter Object Reference") (Duration :type "Float (single-precision)"))
  (`parent.ClientStartBuff` OwningCharacter Duration)
  (bind _asis_base_bpcombat_interface (cast `/Game/Systems/Interfaces/IsBaseBPCombatInterface` (`self.OwningCharacter`)))
  (set `self.ConbatInterface` _asis_base_bpcombat_interface)
  ;[1 1 1] If we didn’t do this; then it would apply the effect twice
  (if (not (`KismetSystemLibrary.IsServer`))
    (goto _label)))

(event `self.GameplayEffectToApplyOnBuffCleared`
  (`ConanCharacter.AddIntStatModifier` (`self.OwningCharacter`) "AttributeAccuracy" "Default" "Add" (* (* (`self.BuffPotency`) 2) -1) "Merge")
  (`parent.GameplayEffectToApplyOnBuffCleared`)
  (`/Game/Systems/Interfaces/IsBaseBPCombatInterface.AdjustMovementSpeedMultiplier` (`self.ConbatInterface`) false (`self.MovementSpeedMultiplier`) :!label _label_2)
  (set `self.MovementSpeedMultiplier` 0.0))

(event `self.ClientClearBuff`
  (params (OwningCharacter :type "ConanCharacter Object Reference"))
  (`parent.ClientClearBuff` OwningCharacter)
  ;[1 1 1] If we didn’t do this; then it would apply the effect twice
  (if (not (`KismetSystemLibrary.IsServer`))
    (goto _label_2)))