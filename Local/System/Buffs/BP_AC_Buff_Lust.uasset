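; Lust buff for player characters that lasts only while an item is equipped in the Torso slot.
; On start it removes itself if that slot is empty, otherwise it listens for equipment removal and clears once the slot empties.
; Its effect lowers NaturalArmor and raises TemperatureModification through additive stat modifiers, reversed on clear.
; The description reports a Charisma increase, which this graph does not apply.
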(event `self.StartBuff`
  (params (BuffPotency :type Integer) (DamageCauser :type "Actor Object Reference") (OwningCharacter :type "ConanCharacter Object Reference") (Instigator :type "Controller Object Reference"))
  (`parent.StartBuff` BuffPotency DamageCauser OwningCharacter Instigator)
  (bind _asbase_player_char (cast `/Game/Characters/BasePlayerChar` OwningCharacter))
  (bind _equipmentinventory (`/Game/Characters/BaseBPChar.EquipmentInventory` _asbase_player_char))
  (`/Engine/EditorBlueprintResources/StandardMacros.IsValid` (`EquipmentInventory.GetItemAtSlot` _equipmentinventory "Torso")
    (:`Is Valid`
      (add `ItemInventory.SignalItemRemoved` _equipmentinventory (delegate `RemovedShirt`)))
    (:`Is Not Valid`
      (`/Game/Systems/Buffs/00_BP_AC_BuffSystem.RemoveBuff` (`/Game/Characters/BaseBPCombat.00_BP_AC_BuffSystem` _asbase_player_char) "BP_AC_Buff_Lust_C" :!label _label))))

(event `RemovedShirt`
  (params (index :type Integer) (item :type "GameItem Object Reference") (dstInventory :type "ItemInventory Object Reference") (dstIndex :type Integer))
  (bind _equipmentinventory (`/Game/Characters/BaseBPChar.EquipmentInventory` (stale `self.StartBuff` _asbase_player_char)))
  (`/Engine/EditorBlueprintResources/StandardMacros.IsValid` (`EquipmentInventory.GetItemAtSlot` _equipmentinventory "Torso")
    (:`Is Not Valid`
      (remove `ItemInventory.SignalItemRemoved` _equipmentinventory (delegate `RemovedShirt`))
      (goto _label))))

(event `self.GameplayEffectToApplyOnBuffStart`
  (bind _owningcharacter (`self.OwningCharacter`))
  (`parent.GameplayEffectToApplyOnBuffStart`)
  (`ConanCharacter.AddFloatStatModifier` _owningcharacter "NaturalArmor" "Default" "Add" -200.0 "Merge")
  (`ConanCharacter.AddFloatStatModifier` _owningcharacter "TemperatureModification" "TimeOfDay" "Add" 130.0 "Merge"))

(event `CustomEvent`)

(event `self.GameplayEffectToApplyOnBuffCleared`
  (bind _owningcharacter (`self.OwningCharacter`))
  (`parent.GameplayEffectToApplyOnBuffCleared`)
  (`ConanCharacter.AddFloatStatModifier` _owningcharacter "NaturalArmor" "Default" "Add" 200.0 "Merge")
  (`ConanCharacter.AddFloatStatModifier` _owningcharacter "TemperatureModification" "TimeOfDay" "Add" -130.0 "Merge"))

(event `CustomEvent_1`)

(fn `GetEffectDescription`
  (returns (Description :type Text))
  (return (`|FormatText` "Charisma increased by 3")))