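; Buff component that temporarily alters the player character's body layout, apparently breast size going by its name.
; On start it caches the current CharacterLayout in Original and applies a rebuilt copy, carrying over the listed scalar parameters rather than the whole struct.
; On clear it restores the cached layout.
; Its description reports a Charisma increase, though these graphs change only appearance.
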(event `self.GameplayEffectToApplyOnBuffStart`
  (bind _asbase_player_char (cast `/Game/Characters/BasePlayerChar` (`self.OwningCharacter`)))
  (bind _character_layout (`/Game/Characters/BasePlayerChar.GetCharacterLayout` _asbase_player_char))
  (bind _output_get (set `self.Original` _character_layout))
  (bind (_meshlayout _texturelayout _tintlayout _boolparams _intparams _scalarparams _enumparams _armourdyeparams) (break `CharacterLayout` _output_get))
  (bind (_height _bust _dick _eyeangle _eyesize _eyedepth _nosewidth _nosesize _nosecurve _jawwidth _cheekheight _cheekwidth _chinwidth _earangle _earsize _lipsize _pitch _physiquemax _physiquemin) (break `CharacterScalarParameters` _scalarparams))
  (`/Game/Characters/BasePlayerChar.SetCharacterLayout` _asbase_player_char (make `CharacterLayout` _meshlayout _texturelayout _tintlayout _boolparams _intparams (make `CharacterScalarParameters` _height 1.0 _dick _eyeangle _eyesize _eyedepth _nosewidth _nosesize _nosecurve _jawwidth _cheekheight _cheekwidth _chinwidth _earangle _earsize _lipsize _pitch _physiquemax _physiquemin) _enumparams _armourdyeparams)))

(event `self.GameplayEffectToApplyOnBuffCleared`
  (bind _asbase_player_char (cast `/Game/Characters/BasePlayerChar` (`self.OwningCharacter`)))
  (`/Game/Characters/BasePlayerChar.SetCharacterLayout` _asbase_player_char (`self.Original`)))

(fn `GetEffectDescription`
  (returns (Description :type Text))
  (return (`|FormatText` "Charisma increased by 3")))