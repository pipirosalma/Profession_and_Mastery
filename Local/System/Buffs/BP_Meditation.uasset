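; Meditation buff that drains a player character's Corruption energy while active.
; On buff start it caches the owning character's energy receiver, and each Tick subtracts a fixed amount, unscaled by delta time, while Corruption is non-negative.
; Client buff clear and EndPlay both call BreakMeditateDMG on the character's AC_SpellCasting_RPC component to break meditation.
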(event `self.ClientClearBuff`
  (params (OwningCharacter :type "ConanCharacter Object Reference"))
  (bind _asbase_player_char (cast `/Game/Characters/BasePlayerChar` OwningCharacter))
  (`/Game/Mods/Profession_and_Mastery/AC_SpellCasting_RPC.BreakMeditate_DMG` (`Actor.GetComponentByClass` _asbase_player_char "/Game/Mods/Profession_and_Mastery/AC_SpellCasting_RPC.AC_SpellCasting_RPC_C") null 0.0 null null null 0)
  (`parent.ClientClearBuff` OwningCharacter))

(event `self.ReceiveEndPlay`
  (params (EndPlayReason :type "EEndPlayReason Enum"))
  (bind _asbase_player_char (cast `/Game/Characters/BasePlayerChar` (`self.OwningCharacter`))
    (:`then`
      (`/Game/Mods/Profession_and_Mastery/AC_SpellCasting_RPC.BreakMeditate_DMG` (`Actor.GetComponentByClass` _asbase_player_char "/Game/Mods/Profession_and_Mastery/AC_SpellCasting_RPC.AC_SpellCasting_RPC_C") null 0.0 null null null 0))
    (:`CastFailed`
      _))
  (`parent.ReceiveEndPlay` EndPlayReason))

(event `self.GameplayEffectToApplyOnBuffStart`
  (bind _asbase_player_char (cast `/Game/Characters/BasePlayerChar` (`self.OwningCharacter`)))
  (set `self.TargetReciver` (`/Game/Characters/BasePlayerChar.BPEnergyReceiver` _asbase_player_char))
  (`parent.GameplayEffectToApplyOnBuffStart`))

(event `self.ReceiveTick`
  (params (DeltaSeconds :type "Float (single-precision)"))
  (bind _targetreciver (`self.TargetReciver`))
  (if (>= (`EnergyReceiverComponent.GetEnergy` _targetreciver "EnergyType_Corruption") 0.0)
    (`EnergyReceiverComponent.ModifyEnergy` _targetreciver "EnergyType_Corruption" -5.0))
  (`parent.ReceiveTick` DeltaSeconds))