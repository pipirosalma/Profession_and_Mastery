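; BP_Fist is the unarmed fist item, which adjusts its damage when equipped by a player of one specific class.
; For that class, OnEquip spawns a Riddle of Steel game item and passes it as a modification kit into light and heavy hit damage modifiers scaled by class level, with heavy slightly higher.
; The parent equip logic then runs, as it does for other owners, but is skipped if the spawned item's cast fails.
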(event `self.OnEquip`
  (params (owner :type "Character Object Reference"))
  (bind _asbase_player_char (cast `/Game/Characters/BasePlayerChar` owner)
    (:`then`
      (bind _returnvalue (`Actor.GetComponentByClass` _asbase_player_char "/Game/Mods/Profession_and_Mastery/AC_Actor_Component_Main.AC_Actor_Component_Main_C"))
      (if (`|EnumEquality` (`/Game/Mods/Profession_and_Mastery/AC_Actor_Component_Main.PlayerClass` _returnvalue) "NewEnumerator0")
        (bind _returnvalue_2 (`GameItemSpawner.SpawnItem` "GameItem" 8995204))
        (bind _asbpgame_item_riddle_of_steel_master (cast `/Game/Systems/RiddleOfSteel/BPGameItem_RiddleOfSteel_Master` _returnvalue_2))
        (bind _returnvalue_3 (+ (* (`/Game/Mods/Profession_and_Mastery/AC_Actor_Component_Main.PlayerClassLevel` _returnvalue) 10) 5))
        (`self.Set Stat Modifiers` self "MaxAttackReach" 0.0 "DamageHealthLight_OnHit" _returnvalue_3 _asbpgame_item_riddle_of_steel_master 1)
        (`self.Set Stat Modifiers` self "MaxAttackReach" 0.0 "DamageHealthHeavy_OnHit" (+ _returnvalue_3 1) _asbpgame_item_riddle_of_steel_master 1)))
    (:`CastFailed`
      _))
  (`parent.OnEquip` owner))