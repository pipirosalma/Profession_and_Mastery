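; Interactable stone that lets a player permanently choose the Entertainer class in a Conan-based game.
; On client activation it reads the player's class from AC_Actor_Component_Main, then shows either a Yes/No prompt or a class-locked notice.
; Accepting calls LearnClassFeat and triggers an effect and multicast sound.
; The non-server confirmation popup says WARRIOR, contradicting the Entertainer prompt.
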(event `InteractableInterface.ClientInteractableActivate`
  (params (Component :type "PrimitiveComponent Object Reference") (Instigator :type "PlayerController Object Reference") (HitIndex :type Integer))
  (bind _asbase_player_char (cast `/Game/Characters/BasePlayerChar` (cast `ConanCharacter` (`Controller.K2_GetPawn` Instigator) :!pure true)))
  (bind _playerclass (`/Game/Mods/Profession_and_Mastery/AC_Actor_Component_Main.PlayerClass` (`self.GetComponentByClass` _asbase_player_char "/Game/Mods/Profession_and_Mastery/AC_Actor_Component_Main.AC_Actor_Component_Main_C")))
  (if (`|EnumEquality` _playerclass "NewEnumerator7")
    (bind _returnvalue (`MessageBoxWidget.CreateMessageBox` self "YesNo" "Class: Entertainer" "Are you sure You want your class to be an ENTERTAINER? \nYOU CAN'T CHANGE ONCE YOU PICK A CLASS "))
    (`MessageBoxWidget.ShowMessageBox` _returnvalue)
    (add `MessageBoxWidget.SignalUserActionPerformed` _returnvalue (delegate `MessageBoxResult`))
    (else
      (bind _returnvalue_2 (`MessageBoxWidget.CreateMessageBox` self "OK" "Class Choice Locked" (`KismetStringLibrary.Concat_StrStr` "You alread have a class:" (`|GetEnumeratorNameAsString` _playerclass))))
      (`MessageBoxWidget.ShowMessageBox` _returnvalue_2))))

(event `MessageBoxResult`
  (params (result :type "EMessageBoxDialogResult Enum"))
  (if (`|EnumEquality` result "Yes")
    (`/Game/Mods/Profession_and_Mastery/AC_Actor_Component_Main.LearnClassFeat` (`self.GetComponentByClass` (stale `InteractableInterface.ClientInteractableActivate` _asbase_player_char) "/Game/Mods/Profession_and_Mastery/AC_Actor_Component_Main.AC_Actor_Component_Main_C") "NewEnumerator1")
    (`ActorComponent.ToggleActive` (`self.Explo`))
    (`ActorComponent.Activate` (`self.BP_BSC_MulticastSound`) false)
    (if (not (`KismetSystemLibrary.IsServer`))
      (bind _returnvalue (`MessageBoxWidget.CreateMessageBox` self "OK" "Class: WARRIOR" "Your class is now WARRIOR"))
      (`MessageBoxWidget.ShowMessageBox` _returnvalue))))

(fn `UserConstructionScript`
  (`parent.UserConstructionScript`))