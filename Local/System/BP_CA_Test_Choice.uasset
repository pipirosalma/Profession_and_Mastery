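; Test interactable actor that teaches the activating player two praying emotes, standing and sitting, through the character's emote controller.
; It also holds class-reset logic: a Yes result calls ClassReset on the player's AC_Actor_Component_Main, then shows an OK message box when not on the server.
; The Yes/No prompt that would bind that handler is disconnected, so activation only grants the emotes.
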(event `InteractableInterface.ClientInteractableActivate`
  (params (Component :type "PrimitiveComponent Object Reference") (Instigator :type "PlayerController Object Reference") (HitIndex :type Integer))
  (bind _asbase_player_char (cast `/Game/Characters/BasePlayerChar` (cast `ConanCharacter` (`Controller.K2_GetPawn` Instigator) :!pure true)))
  (bind _bpemotecontroller (`/Game/Characters/BaseBPCombat.BPEmoteController` _asbase_player_char))
  (`EmoteController.LearnEmote` _bpemotecontroller "PrayStanding" true)
  (`EmoteController.LearnEmote` _bpemotecontroller "PraySitting" true))

(event `MessageBoxResult`
  (params (result :type "EMessageBoxDialogResult Enum"))
  (if (`|EnumEquality` result "Yes")
    (`/Game/Mods/Profession_and_Mastery/AC_Actor_Component_Main.ClassReset` (`self.GetComponentByClass` (stale `InteractableInterface.ClientInteractableActivate` _asbase_player_char) "/Game/Mods/Profession_and_Mastery/AC_Actor_Component_Main.AC_Actor_Component_Main_C"))
    (if (not (`KismetSystemLibrary.IsServer`))
      (bind _returnvalue (`MessageBoxWidget.CreateMessageBox` self "OK" "Class: RESET" "BUGRIS VAGY GECI"))
      (`MessageBoxWidget.ShowMessageBox` _returnvalue))))

(fn `UserConstructionScript`
  (`parent.UserConstructionScript`))