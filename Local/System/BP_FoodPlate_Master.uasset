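; Master Blueprint for an interactable food plate or drink vessel that players fill from their backpack, spike and consume.
; The radial menu offers matching items, or a secret ingredient once filled, passed to AC_ConsumableFillUp.
; A Metabolism-versus-random roll decides whether the label's scent hints at poison or spice.
; Consuming plays a montage, feeds BP_HungerSystem, applies stored buffs and empties it, while TemplateItemID selects visible food meshes.
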(event `self.ReceiveBeginPlay`
  (`self.SetPropsVisibility`)
  (`parent.ReceiveBeginPlay`))

(event `InteractableInterface.InteractableMenu`
  (params (RadialMenu :type "RadialMenu Object Reference") (HitIndex :type Integer))
  (`parent.InteractableMenu` RadialMenu HitIndex)
  (if (`self.IsEmpty`)
    (if (`self.Drinks`)
      (set `self.Type` "drinks")
      (set `self.MenuIcon` "/Game/UI/Textures/GUIs/HUD/HUD_BarAssets/T_DrinkIcon.T_DrinkIcon")
      (else
        (set `self.Type` "food")
        (set `self.MenuIcon` "/Game/UI/Textures/GUIs/HUD/HUD_BarAssets/T_FoodIcon.T_FoodIcon")))
    (else
      (bind _returnvalue (`self.FoodLabelCheck` RadialMenu)
        (:`then`
          (add `RadialMenuEntry.SignalClicked` _returnvalue (delegate `FoodSelection`)))
        (:`RowNotFound`
          _))
      (set `self.Type` "secret ingredient")
      (set `self.MenuIcon` "/Game/UI/Textures/GUIs/HUD/T_BuffIconPoisoned.T_BuffIconPoisoned")))
  (bind _returnvalue_2 (`RadialMenu.AddItem` RadialMenu "Add" (`self.Type`) (`self.MenuIcon`) "None" -1))
  (bind _asbase_player_char (cast `/Game/Characters/BasePlayerChar` (`GameplayStatics.GetPlayerCharacter` 0)))
  (bind _backpackinventory (`/Game/Characters/BasePlayerChar.BackpackInventory` _asbase_player_char))
  (for _index (range (+ (`ItemInventory.MaxItemCount` _backpackinventory) 1))
    (bind _returnvalue_3 (`ItemInventory.GetItem` _backpackinventory _index))
    (`/Engine/EditorBlueprintResources/StandardMacros.IsValid` _returnvalue_3
      (:`Is Valid`
        (bind _templateid (`GameItem.TemplateID` _returnvalue_3))
        (bind _returnvalue_4 (`|GetDataTableRow` "/Game/Items/ItemTable.ItemTable" (`KismetStringLibrary.Conv_StringToName` (`KismetStringLibrary.Conv_IntToString` _templateid)))
          (:`then`
            (if (`self.IsEmpty`)
              (if (`self.Drinks`)
                (bind ((`Name` _name) (`Icon` _icon) (`GUICategory` _guicategory) (`FoodAmount` _foodamount) (`DrinkAmount` _drinkamount)) (break `ItemTableRow` _returnvalue_4))
                (bind _returnvalue_5 (> _foodamount 0))
                (if _returnvalue_5
                  _
                  (elif (> _drinkamount 0)
                    (bind _returnvalue_6 (`RadialMenuEntry.AddSubItem` _returnvalue_2 _name " " (`|ConvertAsset` _icon) "None" -1 :!label _label))
                    (set `RadialMenuEntry.UserValue` _templateid _returnvalue_6)
                    (add `RadialMenuEntry.SignalClicked` _returnvalue_6 (delegate `ConsumableAdded`))))
                (elif _returnvalue_5
                  (goto _label)))
              (elif (`|EnumEquality` _guicategory "Consumable")
                (goto _label))))))))
  (`RadialMenuEntry.AddSubItem` _returnvalue_2 "Cancel" "" "/Game/UI/Textures/GUIs/MainRadialMenu/T_MainRadialMenuIconCancel.T_MainRadialMenuIconCancel" "None" -1))

(event `ConsumableAdded`
  (params (menuEntry :type "RadialMenuEntry Object Reference"))
  (bind _asbase_player_char (cast `/Game/Characters/BasePlayerChar` (`GameplayStatics.GetPlayerCharacter` 0)))
  (`/Game/Mods/Profession_and_Mastery/AC_ConsumableFillUp.ServingConsumable` (`self.GetComponentByClass` _asbase_player_char "/Game/Mods/Profession_and_Mastery/AC_ConsumableFillUp.AC_ConsumableFillUp_C") self (`RadialMenuEntry.UserValue` menuEntry) (not (`self.IsEmpty`)))
  (`GUIModuleController.ActivateModule` (`GUIModuleController.GetGUIModuleController`) "MainRadialMenu" false false))

(event `FoodSelection`
  (params (menuEntry :type "RadialMenuEntry Object Reference"))
  (bind _asbase_player_char (cast `/Game/Characters/BasePlayerChar` (`GameplayStatics.GetPlayerCharacter` 0)))
  (`/Game/Mods/Profession_and_Mastery/AC_ConsumableFillUp.AC_Consume_Food` (`self.GetComponentByClass` _asbase_player_char "/Game/Mods/Profession_and_Mastery/AC_ConsumableFillUp.AC_ConsumableFillUp_C") self)
  (`/Game/Mods/Profession_and_Mastery/AC_Actor_Component_Main.EffectsToPlay` (`self.GetComponentByClass` _asbase_player_char "/Game/Mods/Profession_and_Mastery/AC_Actor_Component_Main.AC_Actor_Component_Main_C") "/Game/Mods/Profession_and_Mastery/Assets/Animation/AM_Eat.AM_Eat" true 0 null (0.0 0.0 0.0) null))

(event `self.InteractableActivate`
  (params (Component :type "PrimitiveComponent Object Reference") (Instigator :type "PlayerController Object Reference") (HitIndex :type Integer))
  (bind _returnvalue (`Controller.K2_GetPawn` (`self.Consumer`)))
  (bind _returnvalue_2 (`self.K2_GetComponentsByClass` _returnvalue "/Game/Systems/Hunger/BP_HungerSystem.BP_HungerSystem_C"))
  (bind _returnvalue_3 (`self.GetComponentByClass` _returnvalue "/Game/Mods/Profession_and_Mastery/AC_Actor_Component_Main.AC_Actor_Component_Main_C"))
  (bind _item (`KismetArrayLibrary.Array_Get` _returnvalue_2))
  (set `self.Consumer` Instigator)
  (if (not (`self.IsEmpty`)) :!label _label_2
    (if (`self.Drinks`)
      (`/Game/Mods/Profession_and_Mastery/AC_Actor_Component_Main.EffectsToPlay` _returnvalue_3 "/Game/Mods/Profession_and_Mastery/Assets/Animation/AM_Drink_F.AM_Drink_F" true 0 null (0.0 0.0 0.0) null)
      (else
        (`/Game/Mods/Profession_and_Mastery/AC_Actor_Component_Main.EffectsToPlay` _returnvalue_3 "/Game/Mods/Profession_and_Mastery/Assets/Animation/AM_Eat.AM_Eat" true 0 null (0.0 0.0 0.0) null)))
    (if (> (`KismetArrayLibrary.Array_Length` _returnvalue_2) 0)
      (`/Game/Systems/Hunger/BP_HungerSystem.ServerDrink` _item (`KismetMathLibrary.Conv_IntToDouble` (`self.DrinkAmount`)))
      (bind _returnvalue_4 (`GameItemSpawner.SpawnGameItem` (`self.TemplateItemID`)))
      (`/Game/Systems/Hunger/BP_HungerSystem.ServerGiveFood` _item _returnvalue_4 0.0)
      (bind _asbase_player_char (cast `/Game/Characters/BasePlayerChar` _returnvalue)
        (:`then`
          (for _array_element (`self.BuffsOnUse`)
            (`/Game/Systems/Buffs/00_BP_AC_BuffSystem.AddBuff` (`/Game/Characters/BaseBPCombat.00_BP_AC_BuffSystem` _asbase_player_char) _array_element null 0 null)))
        (:`CastFailed`
          _)))
    (`self.ResetValues`)
    (`self.SetPropsVisibility`)))

(event `FoodConsume`
  (params (InputPin :type "PlayerController Object Reference"))
  (set `self.Consumer` InputPin)
  (goto _label_2))

(event `CastSetPropsVisibilitySet`
  (bind _returnvalue (not (`self.IsEmpty`)))
  (if (`self.Drinks`) :!label _label_3
    (`SceneComponent.SetVisibility` (`self.FluidSM`) (not (`self.IsEmpty`)) true)
    (else
      (`SceneComponent.SetVisibility` (`self.FoodSM`) false true)
      (if (not (`self.IsEmpty`))
        (switch `string` (`KismetStringLibrary.Conv_IntToString` (`self.TemplateItemID`))
          (:`Default`
            (`SceneComponent.SetVisibility` (`self.chicken`) (not (`self.IsEmpty`)) false))
          (:`13503`
            (`SceneComponent.SetVisibility` (`self.Ham`) (not (`self.IsEmpty`)) false :!label _label_4))
          (:`13540`
            (`SceneComponent.SetVisibility` (`self.Water`) (not (`self.IsEmpty`)) false :!label _label_5))
          (:`13550`
            (`SceneComponent.SetVisibility` (`self.Gruel`) (not (`self.IsEmpty`)) false :!label _label_6))
          (:`13597`
            (goto _label_6))
          (:`13598`
            (goto _label_6))
          (:`13599`
            (goto _label_6))
          (:`13601`
            (goto _label_4))
          (:`18002`
            (`SceneComponent.SetVisibility` (`self.Honey`) (not (`self.IsEmpty`)) false :!label _label_7))
          (:`18206`
            (`SceneComponent.SetVisibility` (`self.Bread`) (not (`self.IsEmpty`)) false :!label _label_8))
          (:`18207`
            (goto _label_4))
          (:`18208`
            (goto _label_4))
          (:`18209`
            (`SceneComponent.SetVisibility` (`self.Egg`) (not (`self.IsEmpty`)) false :!label _label_9))
          (:`18210`
            (goto _label_9))
          (:`18212`
            (goto _label_6))
          (:`18213`
            (goto _label_4))
          (:`18216`
            (`SceneComponent.SetVisibility` (`self.Aloe`) _returnvalue false :!label _label_10)
            (`SceneComponent.SetVisibility` (`self.Water`) _returnvalue false))
          (:`18217`
            (goto _label_4))
          (:`18218`
            (goto _label_6))
          (:`18219`
            (goto _label_9))
          (:`18220`
            (goto _label_9))
          (:`18222`
            (goto _label_10))
          (:`18223`
            (goto _label_4))
          (:`18224`
            (goto _label_5))
          (:`18225`
            (goto _label_10))
          (:`18230`
            (`SceneComponent.SetVisibility` (`self.Egg`) (not (`self.IsEmpty`)) false)
            (`SceneComponent.SetVisibility` (`self.Ham`) (not (`self.IsEmpty`)) false))
          (:`18234`
            (goto _label_6))
          (:`18235`
            (goto _label_5))
          (:`18236`
            (goto _label_10))
          (:`18237`
            (goto _label_5))
          (:`18238`
            (goto _label_10))
          (:`18239`
            (goto _label_5))
          (:`18240`
            (goto _label_5))
          (:`18242`
            (goto _label_4))
          (:`18244`
            (goto _label_4))
          (:`18251`
            (goto _label_4))
          (:`18252`
            (goto _label_6))
          (:`18255`
            (goto _label_9))
          (:`18256`
            (goto _label_9))
          (:`18257`
            (goto _label_9))
          (:`18260`
            (goto _label_4))
          (:`18261`
            (goto _label_9))
          (:`18269`
            (goto _label_7))
          (:`18270`
            (goto _label_6))
          (:`18271`
            (goto _label_7))
          (:`18272`
            (goto _label_4))
          (:`18273`
            (goto _label_8)))))))

(event `SetPropsVisibility`
  (goto _label_3))

(event `ResetValues`
  (set `self.IsEmpty` true)
  (set `self.FoodAmount` 0)
  (set `self.DrinkAmount` 0)
  (set `self.BuffsOnUse` (`|MakeArray` null :!type "/Game/Systems/Buffs/01_BP_AC_Buff_Master Class Reference"))
  (set `self.TemplateItemID` 0))

(fn `UserConstructionScript`
  (`parent.UserConstructionScript`))