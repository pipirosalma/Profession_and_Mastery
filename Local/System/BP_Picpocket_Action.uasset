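; Pickpocket action that lets a player steal two item types from another player's backpack.
; A sphere trace from the head finds the victim, whose drunkenness or level relative to the thief's class level sets difficulty.
; After Yes/No confirmation, a victim buff blocks repeat attempts and random rolls decide success and victim notification.
; The AmountToSteal calculation is unconnected, and items are added to the thief with zero quantity.
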(event `self.OnUseItem`
  (params (invokingCharacter :type "ConanCharacter Object Reference")))

(event `TriggerAction`
  (bind _returnvalue (`Actor.GetComponentByClass` (`self.OwningChar`) "/Script/Engine.SkeletalMeshComponent"))
  (bind _returnvalue_2 (`SceneComponent.GetSocketLocation` _returnvalue "b_head"))
  (bind _asbase_player_char (cast `/Game/Characters/BasePlayerChar` (`self.GetOwner`)))
  (bind _output_get (set `self.OwningChar` _asbase_player_char))
  (set `self.PlayerClassLevel` (`/Game/Mods/Profession_and_Mastery/AC_Actor_Component_Main.PlayerClassLevel` (`Actor.GetComponentByClass` _output_get "/Game/Mods/Profession_and_Mastery/AC_Actor_Component_Main.AC_Actor_Component_Main_C")))
  (bind _outhits (`KismetSystemLibrary.SphereTraceMulti` (+ _returnvalue_2 (0.0 0.0 10.0)) (- (+ (* (`SceneComponent.GetRightVector` _returnvalue) 160) _returnvalue_2) (0.0 0.0 130.0)) 20.0 "TraceTypeQuery1" false (`|MakeArray` (`Controller.K2_GetPawn` (`/Game/Characters/BasePlayerChar.PlayerController` (`self.OwningChar`))) :!type "Actor Object Reference")))
  (bind _asbase_player_char_2 (cast `/Game/Characters/BasePlayerChar` (`.HitActor` (`GameplayStatics.BreakHitResult` (`KismetArrayLibrary.Array_Get` _outhits))))
    (:`then`
      (set `self.VictimBasePlayer` _asbase_player_char_2)
      (set `self.VictimInventory` (`ItemInventory.GetInventoryByType` _asbase_player_char_2 "Backpack"))
      (bind _00_bp_ac_buffsystem (`/Game/Characters/BaseBPCombat.00_BP_AC_BuffSystem` _asbase_player_char_2))
      (if (`/Game/Systems/Buffs/00_BP_AC_BuffSystem.CheckIfBuffExists` _00_bp_ac_buffsystem "/Game/Mods/Profession_and_Mastery/System/Buffs/BP_AC_Buff_PickpocketVictim.BP_AC_Buff_PickpocketVictim_C")
        (message `/Game/Characters/HUDNotification_Interface.NotificationText` (`/Game/Characters/FuncomFunctionLibrary.GetControllerFromActor` (`self.OwningChar`)) "Pickpocket action failed. Try Again later." false)
        (else
          (bind _asbp_ac_buff_drunkenness (cast `/Game/Systems/Buffs/Alcohol/BP_AC_Buff_Drunkenness` (`.BuffComponent` (`/Game/Systems/Buffs/00_BP_AC_BuffSystem.CheckIfBuffExists` _00_bp_ac_buffsystem null)))
            (:`then`
              (if (>= (`/Game/Systems/Buffs/Alcohol/BP_AC_Buff_Drunkenness.DrunkStage` _asbp_ac_buff_drunkenness) 0)
                (set `self.PickpocketDifficulty` 0)
                (bind _returnvalue_3 (`ConanPlayerController.GetCharacterName` (`/Game/Characters/BasePlayerChar.PlayerController` _asbase_player_char_2)))
                (bind _returnvalue_4 (`KismetStringLibrary.Concat_StrStr` "Do you want to sneak into " _returnvalue_3 "'s pocket? \n" _returnvalue_3 " seems to be"))
                (set `self.message` (`KismetStringLibrary.Concat_StrStr` _returnvalue_4 "pretty drunk."))
                (else
                  (bind _returnvalue_5 (/ (`/Game/Systems/Progression/BP_ProgressionSystem.GetLevel` (`KismetArrayLibrary.Array_Get` (`Actor.K2_GetComponentsByClass` _asbase_player_char_2 "/Game/Systems/Progression/BP_ProgressionSystem.BP_ProgressionSystem_C"))) (`self.PlayerClassLevel`)))
                  (if (>= _returnvalue_5 50) :!label _label
                    (set `self.PickpocketDifficulty` 90)
                    (set `self.message` (`KismetStringLibrary.Concat_StrStr` _returnvalue_4 "a nearly impossible target."))
                    (elif (>= _returnvalue_5 30)
                      (set `self.PickpocketDifficulty` 50)
                      (set `self.message` (`KismetStringLibrary.Concat_StrStr` _returnvalue_4 "a challenging target"))
                      (else
                        (set `self.PickpocketDifficulty` 20)
                        (set `self.message` (`KismetStringLibrary.Concat_StrStr` _returnvalue_4 "an easy target."))))))))
            (:`CastFailed`
              (goto _label)))
          (bind _returnvalue_6 (`MessageBoxWidget.CreateMessageBox` (`self.OwningChar`) "YesNo" "Action: Pickpocket" (`self.message`)))
          (`MessageBoxWidget.ShowMessageBox` _returnvalue_6)
          (add `MessageBoxWidget.SignalUserActionPerformed` _returnvalue_6 (delegate `CustomEvent_0`)))))
    (:`CastFailed`
      (message `/Game/Characters/HUDNotification_Interface.NotificationText` (`/Game/Characters/FuncomFunctionLibrary.GetControllerFromActor` (`self.OwningChar`)) "Couldn't find a valid target" false))))

(event `CustomEvent_0`
  (params (result :type "EMessageBoxDialogResult Enum"))
  (bind _victiminventory (`self.VictimInventory`))
  (bind _returnvalue (`ItemInventory.GetInventoryByType` (`ActorComponent.GetOwner` (`Character.CapsuleComponent` (`self.OwningChar`))) "Backpack"))
  (bind _returnvalue_2 (`ItemInventory.GetInventoryByType` (`ActorComponent.GetOwner` (`Character.CapsuleComponent` (`self.OwningChar`))) "Backpack"))
  (if (`|EnumEquality` result "Yes")
    (`/Game/Systems/Buffs/00_BP_AC_BuffSystem.AddBuff` (`/Game/Characters/BaseBPCombat.00_BP_AC_BuffSystem` (`self.VictimBasePlayer`)) "/Game/Mods/Profession_and_Mastery/System/Buffs/BP_AC_Buff_PickpocketVictim.BP_AC_Buff_PickpocketVictim_C" null 0 null)
    (if (<= (`self.PickpocketDifficulty`) (`KismetMathLibrary.RandomIntegerInRange` 0 100))
      (`ItemInventory.ValidatedDeleteItemsByTemplate` _victiminventory 11066 (`self.AmountToSteal` _victiminventory 11066))
      (`ItemInventory.AddItemTemplate` _returnvalue 11066 (`ItemInventory.GetFirstFreeIndex` _returnvalue false) 0 false 1.0 1.0)
      (`ItemInventory.ValidatedDeleteItemsByTemplate` _victiminventory 11065 (`self.AmountToSteal` _victiminventory 11065))
      (`ItemInventory.AddItemTemplate` _returnvalue_2 11065 (`ItemInventory.GetFirstFreeIndex` _returnvalue_2 false) 0 false 1.0 1.0)
      (if (<= (`self.PickpocketDifficulty`) (`KismetMathLibrary.RandomIntegerInRange` 0 100))
        (message `/Game/Characters/HUDNotification_Interface.NotificationText` (`/Game/Characters/FuncomFunctionLibrary.GetControllerFromActor` (`self.VictimBasePlayer`)) "Your pocket feels lighter." false))
      (else
        (message `/Game/Characters/HUDNotification_Interface.NotificationText` (`/Game/Characters/FuncomFunctionLibrary.GetControllerFromActor` (`self.OwningChar`)) "Pickpocket action failed" false)))))