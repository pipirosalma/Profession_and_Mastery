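; BP_Nomad_Loot_Crate is a usable loot crate item that grants the player random rewards.
; On use, the server rolls a few rows from the high-quality and low-quality loot DataTables, picking indices from 1 to row count, so row zero is skipped.
; GiveItem adds each randomized quantity to the backpack via AC_Actor_Component_Main.
; Parent OnUseItem runs after server rolls or a failed player cast.
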(event `self.OnUseItem`
  (params (invokingCharacter :type "ConanCharacter Object Reference"))
  (bind _asbase_player_char (cast `/Game/Characters/BasePlayerChar` invokingCharacter)
    (:`then`
      (set `self.InteractingBasePlayerChar` _asbase_player_char)
      (if (`KismetSystemLibrary.IsServer`)
        (for _ (range 1 (+ (`KismetMathLibrary.RandomIntegerInRange` 1 2) 1))
          (bind _outrownames (`DataTableFunctionLibrary.GetDataTableRowNames` "/Game/Mods/Profession_and_Mastery/System/Merchants/db_LootCrate_HQ.db_LootCrate_HQ"))
          (bind _returnvalue (`|GetDataTableRow` "/Game/Mods/Profession_and_Mastery/System/Merchants/db_LootCrate_HQ.db_LootCrate_HQ" (`KismetArrayLibrary.Array_Get` _outrownames (`KismetMathLibrary.RandomIntegerInRange` 1 (`KismetArrayLibrary.Array_Length` _outrownames))))
            (:`then`
              (bind ((`RewardID_4_FE087622492E63229C466BA84B7FD9D5` _rewardid) (`MinimumQuantity_6_7B081F53426CC474969137AA23039F64` _minimumquantity) (`MAximumQuantity_8_6E8C13FC489C04CF67045EB1CCBDD198` _maximumquantity)) (break `/Game/Mods/Profession_and_Mastery/System/Merchants/LootCrate` _returnvalue))
              (`self.GiveItem` _rewardid (`KismetMathLibrary.RandomIntegerInRange` _minimumquantity _maximumquantity)))))
        (for _ (range 1 (+ (`KismetMathLibrary.RandomIntegerInRange` 1 3) 1))
          (bind _outrownames_2 (`DataTableFunctionLibrary.GetDataTableRowNames` "/Game/Mods/Profession_and_Mastery/System/Merchants/db_LootCrate_LQ.db_LootCrate_LQ"))
          (bind _returnvalue_2 (`|GetDataTableRow` "/Game/Mods/Profession_and_Mastery/System/Merchants/db_LootCrate_LQ.db_LootCrate_LQ" (`KismetArrayLibrary.Array_Get` _outrownames_2 (`KismetMathLibrary.RandomIntegerInRange` 1 (`KismetArrayLibrary.Array_Length` _outrownames_2))))
            (:`then`
              (bind ((`RewardID_4_FE087622492E63229C466BA84B7FD9D5` _rewardid_2) (`MinimumQuantity_6_7B081F53426CC474969137AA23039F64` _minimumquantity_2) (`MAximumQuantity_8_6E8C13FC489C04CF67045EB1CCBDD198` _maximumquantity_2)) (break `/Game/Mods/Profession_and_Mastery/System/Merchants/LootCrate` _returnvalue_2))
              (`self.GiveItem` _rewardid_2 (`KismetMathLibrary.RandomIntegerInRange` _minimumquantity_2 _maximumquantity_2)))))
        (`parent.OnUseItem` invokingCharacter :!label _label)))
    (:`CastFailed`
      (goto _label))))