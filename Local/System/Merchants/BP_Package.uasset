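; Merchant package item Blueprint that changes the wearer's buffs and perks while equipped.
; Equipping adds the BP_Caravan buff to the player character's buff system, and unequipping removes it.
; For one player class, equipping also grants the Encumberance_50 perk, while unequipping removes Agility_50 and rechecks Encumberance_50.
; Both events then call their parent implementations.
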(event `self.OnEquip`
  (params (owner :type "Character Object Reference"))
  (bind _asbase_player_char (cast `/Game/Characters/BasePlayerChar` owner))
  (`/Game/Systems/Buffs/00_BP_AC_BuffSystem.AddBuff` (`/Game/Characters/BaseBPCombat.00_BP_AC_BuffSystem` _asbase_player_char) "/Game/Mods/Profession_and_Mastery/System/Merchants/BP_Caravan.BP_Caravan_C" null 0 null)
  (if (`|EnumEquality` (`/Game/Mods/Profession_and_Mastery/AC_Actor_Component_Main.PlayerClass` (`Actor.GetComponentByClass` _asbase_player_char "/Game/Mods/Profession_and_Mastery/AC_Actor_Component_Main.AC_Actor_Component_Main_C")) "NewEnumerator6")
    (`/Game/Characters/BaseBPChar.GetFootstepSoundType` _asbase_player_char)
    (`PerkSystemComponent.AddOwnedPerk` (`/Game/Characters/BasePlayerChar.BP_PerkSystemComponent` _asbase_player_char) "Encumberance_50"))
  (`parent.OnEquip` owner))

(event `self.OnUnEquip`
  (params (owner :type "Character Object Reference"))
  (bind _asbase_player_char (cast `/Game/Characters/BasePlayerChar` owner)
    (:`then`
      (`/Game/Systems/Buffs/00_BP_AC_BuffSystem.RemoveBuff` (`/Game/Characters/BaseBPCombat.00_BP_AC_BuffSystem` _asbase_player_char) "/Game/Mods/Profession_and_Mastery/System/Merchants/BP_Caravan.BP_Caravan_C"))
    (:`CastFailed`
      _))
  (if (`|EnumEquality` (`/Game/Mods/Profession_and_Mastery/AC_Actor_Component_Main.PlayerClass` (`Actor.GetComponentByClass` _asbase_player_char "/Game/Mods/Profession_and_Mastery/AC_Actor_Component_Main.AC_Actor_Component_Main_C")) "NewEnumerator6")
    (bind _bp_perksystemcomponent (`/Game/Characters/BasePlayerChar.BP_PerkSystemComponent` _asbase_player_char))
    (`PerkSystemComponent.RemoveOwnedPerk` _bp_perksystemcomponent "Agility_50")
    (`/Game/Systems/Perks/BP_PerkSystemComponent.CheckAndApplyPerk` _bp_perksystemcomponent "Encumberance_50"))
  (`parent.OnUnEquip` owner))