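; Merchant trade actor that buys and sells trade-good shipments through confirmation message boxes when a player interacts with it.
; A head-slot item found in PrioList gets a sale offer at its mapped price; otherwise only one player class can buy a shipment.
; Purchase checks equipment inventory for gold and silver but deducts from the backpack.
; Selling removes the head item, but its backpack payout has no item or amount set.
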(event `InteractableInterface.ClientInteractableActivate`
  (params (Component :type "PrimitiveComponent Object Reference") (Instigator :type "PlayerController Object Reference") (HitIndex :type Integer))
  (bind _tradegoods (`self.TradeGoods`))
  (bind _asbase_player_char (cast `/Game/Characters/BasePlayerChar` (cast `ConanCharacter` (`Controller.K2_GetPawn` Instigator) :!pure true)))
  (set `self.InteractingBasePlayerChar` _asbase_player_char)
  (bind _templateid (`GameItem.TemplateID` (`EquipmentInventory.GetItemAtSlot` (`/Game/Characters/BaseBPChar.GetEquipmentInventory` _asbase_player_char) "Head")))
  (bind (_value _returnvalue) (`BlueprintMapLibrary.Map_Find` (`self.PrioList`) _templateid))
  (if _returnvalue
    (bind _returnvalue_2 (`|GetDataTableRow` "/Game/Mods/Profession_and_Mastery/DataTables/dt_Class_Mastery_Item_Table.dt_Class_Mastery_Item_Table" (`KismetSystemLibrary.MakeLiteralName` (`KismetStringLibrary.Conv_StringToName` (`KismetStringLibrary.Conv_IntToString` _templateid))))
      (:`then`
        (bind _returnvalue_3 (`MessageBoxWidget.CreateMessageBox` self "YesNo" "Supliments" (`KismetStringLibrary.Concat_StrStr` "Would you like to sell the" (`KismetTextLibrary.Conv_TextToString` (`.Name` (break `ItemTableRow` _returnvalue_2))) "for" (`KismetStringLibrary.Conv_IntToString` _value) "gold coins?")))
        (`MessageBoxWidget.ShowMessageBox` _returnvalue_3)
        (add `MessageBoxWidget.SignalUserActionPerformed` _returnvalue_3 (delegate `SellShipment`))))
    (elif (`|EnumEquality` (`/Game/Mods/Profession_and_Mastery/AC_Actor_Component_Main.PlayerClass` (`self.GetComponentByClass` _asbase_player_char "/Game/Mods/Profession_and_Mastery/AC_Actor_Component_Main.AC_Actor_Component_Main_C")) "NewEnumerator6")
      (bind _returnvalue_4 (`MessageBoxWidget.CreateMessageBox` self "YesNo" (`KismetStringLibrary.Concat_StrStr` _tradegoods "trader") (`KismetStringLibrary.Concat_StrStr` "Would you like to purchase a shipment of" _tradegoods " for 10 gold and 50 silver coins? ")))
      (`MessageBoxWidget.ShowMessageBox` _returnvalue_4)
      (add `MessageBoxWidget.SignalUserActionPerformed` _returnvalue_4 (delegate `PurchaseShipment`))
      (else
        (bind _returnvalue_5 (`MessageBoxWidget.CreateMessageBox` self "OK" "Nothing to trade" "You got no business here, be on your way."))
        (`MessageBoxWidget.ShowMessageBox` _returnvalue_5)))))

(event `SellShipment`
  (params (result :type "EMessageBoxDialogResult Enum"))
  (bind _inventory (`/Game/Characters/BaseBPChar.GetEquipmentInventory` (`self.InteractingBasePlayerChar`)))
  (if (`|EnumEquality` result "Yes")
    (`ItemInventory.RemoveItem` _inventory (`EquipmentInventory.GetSlotIndex` _inventory "Head"))
    (bind _returnvalue (`ConanCharacter.GetBackpackInventory` (`self.InteractingBasePlayerChar`)))
    (`ItemInventory.AddItemTemplate` _returnvalue 0 0 1 true 1.0 -1.0)))

(event `PurchaseShipment`
  (params (result :type "EMessageBoxDialogResult Enum"))
  (bind _equipmentinventory (`/Game/Characters/BaseBPChar.EquipmentInventory` (`self.InteractingBasePlayerChar`)))
  (if (`|EnumEquality` result "Yes")
    (`/Game/Systems/BP_MacroGlobal.And+Branch` (`ItemInventory.HasItemByTemplateID` _equipmentinventory (`self.GOLD`) 10) (`ItemInventory.HasItemByTemplateID` _equipmentinventory (`self.SILVER`) 50) ; Quest2 Item Check
      (:`True`
        (bind _returnvalue (`ConanCharacter.GetBackpackInventory` (`self.InteractingBasePlayerChar`)))
        (`|ExecutionSequence`
          (:`then_0`
            (`ItemInventory.AddItemTemplate` _returnvalue (`self.TradeGoodsID`) (`ItemInventory.GetFirstFreeIndex` _returnvalue false) 1 true 1.0 -1.0))
          (:`then_1`
            (`ItemInventory.ValidatedDeleteItemsByTemplate` _returnvalue (`self.GOLD`) 10))
          (:`then_2`
            (`ItemInventory.ValidatedDeleteItemsByTemplate` _returnvalue (`self.SILVER`) 50))))
      (:`False`
        (bind _returnvalue_2 (`MessageBoxWidget.CreateMessageBox` self "OK" "Insufficient funds" "You don't have enough money to purchase this package"))
        (`MessageBoxWidget.ShowMessageBox` _returnvalue_2)))))

(fn `UserConstructionScript`
  (`parent.UserConstructionScript`))