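; Interactable quest-giver NPC "Pedro Paramo" that offers archery and hunting trade-in quests to Conan players.
; On interaction it checks the player's backpack for both Quest 2 items and completes that quest, otherwise shows the quest description.
; Completion deletes required items, then grants a reward and story message, or notifies an error if either deletion fails.
; Quest 1's completion function exists, but its check is hardwired false and never calls it.
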(event `InteractableInterface.InteractableActivate`
  (params (Component :type "PrimitiveComponent Object Reference") (Instigator :type "PlayerController Object Reference") (HitIndex :type Integer))
  (set `self.Saved_instigator` Instigator)
  (bind _asconan_character (cast `ConanCharacter` (`Controller.K2_GetPawn` Instigator))
    (:`then`
      (bind _output_get (set `self.ConChar` _asconan_character))
      (bind _returnvalue (`ConanCharacter.GetBackpackInventory` _output_get))
      (bind _output_get_2 (set `self.PlayerInvRef` _returnvalue))
      (`/Game/Systems/BP_MacroGlobal.And+Branch` false ; Quest1 Item Check
        (:`False`
          ;[1 1 1] Q2 Requirements
          (`/Game/Systems/BP_MacroGlobal.And+Branch` (`ItemInventory.HasItemByTemplateID` _output_get_2 (`self.Q2 R 1 ID`) (`self.Q2 R 1 Q`)) (`ItemInventory.HasItemByTemplateID` _output_get_2 (`self.Q2 R 2 ID`) (`self.Q2 R 2 Q`)) ; Quest2 Item Check
            (:`True`
              (`self.Quest_2_Complete`))
            (:`False`
              (`ConanCharacter.ClientShowMessage` (`self.ConChar`) "Pedro Paramo" "An man with weary eyes, tired muscles, and a skin grained by the constant rain of sand looks at you as you approach. He’s removing a bullseye drawing from an archery target with a perfect shot. Proud to his personal accomplishment, he shares his happiness with you with a grin.\n\n“You will need a thousand shots to beat that!” \nHe says, pointing the perfect hole mark in the center of the bulls eye... “Bring enough arrows, and I could teach you!”\n\n\nHe lifts his hand and signals to wait “Once you’re ready, or if you feel you can beat that… Bring me ten heads of a mighty Black Rhino!”\n\n((1000 Razor Arrows and 100 silver))\n((10 Black Rhino Heads and 250 golds))\n" :!pinned true) ; Both Quest Requ is missing
            )))))
    (:`CastFailed`
      (`KismetSystemLibrary.PrintString` "Casto to Conan Character Failed"))))

(event `self.ReceiveBeginPlay`
  (`/Game/Systems/Building/BuildingActorComponents/BP_BAC_TurnLightOnOff.TurnOnAll` (`self.BP_BAC_TurnLightOnOff`))
  (`parent.ReceiveBeginPlay`))

(fn `GetArtisanThrallInventory`
  (returns (ReturnValue :type "ItemInventory Object Reference"))
  (return (`self.ThrallInventory`)))

(fn `Quest_1_Complete`
  (bind _playerinvref (`self.PlayerInvRef`))
  (bind _saved_instigator (`self.Saved_instigator`))
  (bind _success (`/Game/Systems/MiscFunctions.DeleteItemsInAllInventoriesByTemplateID` _saved_instigator (`self.Q1_R_ID`) (`self.Q1 R Q`)))
  (bind _success_2 (`/Game/Systems/MiscFunctions.DeleteItemsInAllInventoriesByTemplateID` _saved_instigator (`self.Q1 R 2 ID`) (`self.Q1 R 2 Q`)))
  (`/Game/Systems/BP_MacroGlobal.And+Branch` _success_2 _success
    (:`True`
      (`ItemInventory.AddItemTemplate` _playerinvref (`self.Q1 Reward`) (`ItemInventory.GetFirstFreeIndex` _playerinvref false) 1 false 1.0 -1.0 :!pinned true) ; Reward
      (`ConanCharacter.ClientShowMessage` (`self.ConChar`) "Bull’s eye Souvenir" "Once you come with the arrows, the training starts. The man is kind, and teaches you the secrets of archery with an unnatural clarity. After a couple of days, you leave with a new friend, and the token of your achievement. In the form of a bullseye painting." :!pinned true) ; Complete Text
    )
    (:`False`
      (bind _asfun_combat_player_controller (cast `/Game/Systems/FunCombat_PlayerController` _saved_instigator))
      (`/Game/Systems/FunCombat_PlayerController.NotificationText` _asfun_combat_player_controller "Quest Error" false))))

(fn `Quest_2_Complete`
  (bind _playerinvref (`self.PlayerInvRef`))
  (bind _saved_instigator (`self.Saved_instigator`))
  (bind _success (`/Game/Systems/MiscFunctions.DeleteItemsInAllInventoriesByTemplateID` _saved_instigator (`self.Q2 R 1 ID`) (`self.Q2 R 1 Q`)))
  (bind _success_2 (`/Game/Systems/MiscFunctions.DeleteItemsInAllInventoriesByTemplateID` _saved_instigator (`self.Q2 R 2 ID`) (`self.Q2 R 2 Q`)))
  (`/Game/Systems/BP_MacroGlobal.And+Branch` _success_2 _success
    (:`True`
      (`ItemInventory.AddItemTemplate` _playerinvref (`self.Q2 Reward`) (`ItemInventory.GetFirstFreeIndex` _playerinvref false) 1 false 1.0 -1.0 :!pinned true) ; Reward
      (`ConanCharacter.ClientShowMessage` (`self.ConChar`) "Hunter’s Prowess" "“Well look what your training did! I can only say I’m impressed. Take this Bow leather handle grip, it will wear out, like they all do… but it will teach you something.” The man walks away, chuckling with charm, disappears in the distance.\n" :!pinned true) ; Complete Text
    )
    (:`False`
      (bind _asfun_combat_player_controller (cast `/Game/Systems/FunCombat_PlayerController` _saved_instigator))
      (`/Game/Systems/FunCombat_PlayerController.NotificationText` _asfun_combat_player_controller "Quest Error" false))))

(fn `UserConstructionScript`
  (`parent.UserConstructionScript`))