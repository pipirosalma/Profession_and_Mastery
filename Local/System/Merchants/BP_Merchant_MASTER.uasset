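; Master Blueprint for merchants who trade shipments with players for gold and silver through message boxes on interaction.
; Its SellItemID row in Dt_NomadTradePrice supplies MerchantData, from which MakeAnOffer picks each shipment type's price.
; A head-slot item found in that table prompts a sale, paying coins plus an extra item.
; Otherwise only one player class may buy the merchant's shipment, after a backpack funds check; others are turned away.
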(event `InteractableInterface.ClientInteractableActivate`
  (params (Component :type "PrimitiveComponent Object Reference") (Instigator :type "PlayerController Object Reference") (HitIndex :type Integer))
  (bind _returnvalue (`Controller.K2_GetPawn` Instigator))
  (bind _offeredprice (`self.OfferedPrice`))
  (bind _asconan_character (cast `ConanCharacter` _returnvalue :!pure true))
  (bind _returnvalue_2 (`|GetDataTableRow` "/Game/Mods/Profession_and_Mastery/DataTables/dt_NomadTradePrice.dt_NomadTradePrice" (`self.SellItemID`))
    (:`then`
      (set `self.MerchantData` _returnvalue_2)
      (set `self.MsgTarget` _asconan_character)
      (bind _asbase_player_char (cast `/Game/Characters/BasePlayerChar` _asconan_character))
      (set `self.InteractingBasePlayerChar` _asbase_player_char)
      (bind _templateid (`GameItem.TemplateID` (`EquipmentInventory.GetItemAtSlot` (`/Game/Characters/BaseBPChar.GetEquipmentInventory` _asbase_player_char) "Head")))
      (`|GetDataTableRow` "/Game/Mods/Profession_and_Mastery/DataTables/dt_NomadTradePrice.dt_NomadTradePrice" (`KismetStringLibrary.Conv_StringToName` (`KismetStringLibrary.Conv_IntToString` _templateid))
        (:`then`
          (bind (_sellitemname _output_get) (`self.MakeAnOffer` _templateid))
          (bind _returnvalue_3 (`MessageBoxWidget.CreateMessageBox` (`self.MsgTarget`) "YesNo" "Merchant" (`KismetStringLibrary.Concat_StrStr` "Would you like to sell the " _sellitemname "for" (`KismetStringLibrary.Concat_StrStr` (`KismetStringLibrary.Conv_IntToString` (`KismetArrayLibrary.Array_Get` _output_get)) " gold and " (`KismetStringLibrary.Conv_IntToString` (`KismetArrayLibrary.Array_Get` _output_get 1)) " silver coins?"))))
          (`MessageBoxWidget.ShowMessageBox` _returnvalue_3)
          (add `MessageBoxWidget.SignalUserActionPerformed` _returnvalue_3 (delegate `SellShipment`)))
        (:`RowNotFound`
          (if (`|EnumEquality` (`/Game/Mods/Profession_and_Mastery/AC_Actor_Component_Main.PlayerClass` (`self.GetComponentByClass` _asbase_player_char "/Game/Mods/Profession_and_Mastery/AC_Actor_Component_Main.AC_Actor_Component_Main_C")) "NewEnumerator6")
            (bind _sellitemname_2 (`self.MakeAnOffer` (`KismetStringLibrary.Conv_StringToInt` (`KismetStringLibrary.Conv_NameToString` (`self.SellItemID`)))))
            (bind _returnvalue_4 (`MessageBoxWidget.CreateMessageBox` _returnvalue "YesNo" (`KismetStringLibrary.Concat_StrStr` _sellitemname_2 "trader") (`KismetStringLibrary.Concat_StrStr` "Would you like to purchase a shipment of" _sellitemname_2 " for " (`KismetStringLibrary.Concat_StrStr` (`KismetStringLibrary.Conv_IntToString` (`KismetArrayLibrary.Array_Get` _offeredprice)) " gold and " (`KismetStringLibrary.Conv_IntToString` (`KismetArrayLibrary.Array_Get` _offeredprice 1)) " silver coins?"))))
            (`MessageBoxWidget.ShowMessageBox` _returnvalue_4)
            (add `MessageBoxWidget.SignalUserActionPerformed` _returnvalue_4 (delegate `PurchaseShipment`))
            (else
              (bind _returnvalue_5 (`MessageBoxWidget.CreateMessageBox` _asbase_player_char "OK" "Nothing to trade" "You got no business here, be on your way."))
              (`MessageBoxWidget.ShowMessageBox` _returnvalue_5))))))))

(event `SellShipment`
  (params (result :type "EMessageBoxDialogResult Enum"))
  (bind _offeredprice (`self.OfferedPrice`))
  (bind _inventory (`/Game/Characters/BaseBPChar.GetEquipmentInventory` (`self.InteractingBasePlayerChar`)))
  (if (`|EnumEquality` result "Yes")
    (`ItemInventory.RemoveItem` _inventory (`EquipmentInventory.GetSlotIndex` _inventory "Head"))
    (`self.GiveItem` (`self.GOLD`) (`KismetArrayLibrary.Array_Get` _offeredprice))
    (`self.GiveItem` (`self.SILVER`) (`KismetArrayLibrary.Array_Get` _offeredprice 1))
    (`self.GiveItem` 8941812 1)))

(event `PurchaseShipment`
  (params (result :type "EMessageBoxDialogResult Enum"))
  (bind _offeredprice (`self.OfferedPrice`))
  (bind _offeredprice_2 (`self.OfferedPrice`))
  (bind _backpackinventory (`/Game/Characters/BasePlayerChar.BackpackInventory` (`self.InteractingBasePlayerChar`)))
  (if (`|EnumEquality` result "Yes")
    (`/Game/Systems/BP_MacroGlobal.And+Branch` (`ItemInventory.HasItemByTemplateID` _backpackinventory (`self.GOLD`) (`KismetArrayLibrary.Array_Get` _offeredprice_2)) (`ItemInventory.HasItemByTemplateID` _backpackinventory (`self.SILVER`) (`KismetArrayLibrary.Array_Get` _offeredprice_2 1)) ; Quest2 Item Check
      (:`True`
        (bind _returnvalue (`ConanCharacter.GetBackpackInventory` (`self.InteractingBasePlayerChar`)))
        (`|ExecutionSequence`
          (:`then_0`
            (`self.GiveItem` (`KismetStringLibrary.Conv_StringToInt` (`KismetStringLibrary.Conv_NameToString` (`self.SellItemID`))) 1))
          (:`then_1`
            (`ItemInventory.ValidatedDeleteItemsByTemplate` _returnvalue (`self.GOLD`) (`KismetArrayLibrary.Array_Get` _offeredprice)))
          (:`then_2`
            (`ItemInventory.ValidatedDeleteItemsByTemplate` _returnvalue (`self.SILVER`) (`KismetArrayLibrary.Array_Get` _offeredprice 1)))))
      (:`False`
        (bind _returnvalue_2 (`MessageBoxWidget.CreateMessageBox` (`self.MsgTarget`) "OK" "Insufficient funds" "You don't have enough money to purchase this package"))
        (`MessageBoxWidget.ShowMessageBox` _returnvalue_2)))))

(fn `UserConstructionScript`
  (`parent.UserConstructionScript`))