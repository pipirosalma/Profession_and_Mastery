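; BP_Love_potion is a spell buff that makes its owner "madly in love" with a character they look at.
; Until a lover is found, Tick and client buff ticks run a debug-drawn sphere trace from the head bone along the mesh's right vector.
; If the first hit is a player character, the buff is renamed with their name.
; It then gets a random duration and a refreshed widget, and searching stops.
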(event `self.ReceiveBeginPlay`)

(event `SearchYourLove`
  (bind _asbase_player_char (cast `/Game/Characters/BasePlayerChar` (`self.OwningCharacter`)))
  (bind _returnvalue (`Actor.GetComponentByClass` _asbase_player_char "/Script/Engine.SkeletalMeshComponent"))
  (bind _returnvalue_2 (`SceneComponent.GetSocketLocation` _returnvalue "b_head"))
  (bind _outhits (`KismetSystemLibrary.SphereTraceMulti` (+ _returnvalue_2 (0.0 0.0 10.0)) (+ (* (`SceneComponent.GetRightVector` _returnvalue) 500) _returnvalue_2) 140.0 "TraceTypeQuery1" false (`|MakeArray` (`Controller.K2_GetPawn` (`/Game/Characters/BasePlayerChar.PlayerController` _asbase_player_char)) :!type "Actor Object Reference") "ForDuration"))
  (bind _asbase_player_char_2 (cast `/Game/Characters/BasePlayerChar` (`.HitActor` (`GameplayStatics.BreakHitResult` (`KismetArrayLibrary.Array_Get` _outhits)))))
  (set `self.Name` (`KismetTextLibrary.Conv_StringToText` (`KismetStringLibrary.Concat_StrStr` "Madly in love with" (`/Game/Characters/BaseBPChar.CharacterName` _asbase_player_char_2))))
  (`self.UpdateClients`)
  (set `self.HasLover` true))

(event `self.ClientDoBuffTick`
  (if (not (`self.HasLover`)) :!label _label
    (`self.SearchYourLove`)))

(event `self.ReceiveTick`
  (params (DeltaSeconds :type "Float (single-precision)"))
  (goto _label))

(event `UpdateClients`
  (if (not (`self.HasLover`))
    (bind _output_get (set `self.BuffTicks` (`KismetMathLibrary.RandomIntegerInRange` 300 18000)))
    (set `self.BuffTicks_Remaining` _output_get)
    (`|ExecutionSequence`
      (:`then_0`
        (if (not (`KismetSystemLibrary.IsDedicatedServer`))
          (`self.RemoveBuffWidget`)))
      (:`then_1`
        (set `self.HasLover` true)
        (`self.AddBuffWidget` (* (`self.BuffTicks_Remaining`) (`self.BuffTickDuration`)))))))