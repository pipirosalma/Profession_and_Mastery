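; BP_GlomyAura is a spell buff that gives the owning player character an undead head.
; Buff start, both start-effect events and Tick share one path: cache current meshes in SavedData, swap only Head to SK_undead, update meshes.
; ClearBuff reapplies SavedData through the customization component.
; Because every tick overwrites SavedData, the cache can capture the undead head instead of the original.
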(event `self.ReceiveTick`
  (params (DeltaSeconds :type "Float (single-precision)"))
  (bind _asbase_player_char (cast `/Game/Characters/BasePlayerChar` (`self.OwningCharacter`) :!label _label))
  (bind _bp_charactercustomizationcomponent (`/Game/Characters/BasePlayerChar.BP_CharacterCustomizationComponent` _asbase_player_char))
  (bind _meshes (`CharacterCustomizationComponent.Meshes` _bp_charactercustomizationcomponent))
  (set `self.SavedData` _meshes)
  (bind (_helmet _hair _facialhair _head _forearms _hands _upperbody _lowerbody _legs _feet) (break `CharacterResolvedMeshes` _meshes))
  (`CharacterCustomizationComponent.SetMeshes` _bp_charactercustomizationcomponent (make `CharacterResolvedMeshes` _helmet _hair _facialhair "/Game/Characters/NPCs/Undead/Meshes/SK_undead.SK_undead" _forearms _hands _upperbody _lowerbody _legs _feet) true)
  (`/Game/Characters/BasePlayerChar.UpdateMeshes` _asbase_player_char))

(event `self.StartBuff`
  (params (BuffPotency :type Integer) (DamageCauser :type "Actor Object Reference") (OwningCharacter :type "ConanCharacter Object Reference") (Instigator :type "Controller Object Reference"))
  (`parent.StartBuff` BuffPotency DamageCauser OwningCharacter Instigator)
  (goto _label))

(event `self.GameplayEffectToApplyOnBuffStart`
  (goto _label))

(event `self.VisualEffectToApplyOnBuffStart`
  (goto _label))

(event `self.ClearBuff`
  (bind _asbase_player_char (cast `/Game/Characters/BasePlayerChar` (`self.OwningCharacter`)))
  (`CharacterCustomizationComponent.SetMeshes` (`/Game/Characters/BasePlayerChar.BP_CharacterCustomizationComponent` _asbase_player_char) (`self.SavedData`) true)
  (`/Game/Characters/BasePlayerChar.UpdateMeshes` _asbase_player_char))