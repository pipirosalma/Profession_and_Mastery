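; Cursed land curio that radiates an energy source and particle effect until cleansed, and punishes its destruction while still cursed.
; Tick counts down its duration and triggers Cleansing at zero, which removes the energy source and effect; BeginPlay strips both if not cursed.
; Destroying it while cursed activates an explosion, adding capped corruption and a bleeding buff to nearby pawns found through the world settings' player pawn registry.
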(event `Cleansing`
  (`ActorComponent.K2_DestroyComponent` (`self.EnergySource`))
  (`ActorComponent.Deactivate` (`self.ParticleSystem`))
  (set `self.Cursed` false))

(event `self.ReceiveTick`
  (params (DeltaSeconds :type "Float (single-precision)"))
  (bind _output_get (set `self.DurationInSeconds` (- (`self.DurationInSeconds`) 1800)))
  (if (>= 0 _output_get)
    (`self.Cleansing`))
  (`parent.ReceiveTick` 0.0))

(event `self.ReceiveBeginPlay`
  (if (not (`self.Cursed`))
    (`ActorComponent.K2_DestroyComponent` (`self.EnergySource`))
    (`ActorComponent.Deactivate` (`self.ParticleSystem`)))
  (`parent.ReceiveBeginPlay`))

(event `self.ReceiveDestroyed`
  (if (`self.Cursed`)
    (`ActorComponent.Activate` (`self.explosion`) false)
    (bind _outactors (`GameplayStatics.GetAllActorsOfClass` "/Script/ConanSandbox.ConanWorldSettings"))
    (bind _returnvalue (`ConanWorldSettings.GetPlayerPawnRegistry` (`KismetArrayLibrary.Array_Get` _outactors)))
    (bind _returnvalue_2 (`PlayerPawnRegistry.GetPawnsWithinDistance` _returnvalue (`self.K2_GetActorLocation` self) 500.0))
    (for _array_element _returnvalue_2
      (bind _returnvalue_3 (`self.K2_GetComponentsByClass` _array_element "/Game/Systems/BPEnergyReceiver.BPEnergyReceiver_C"))
      (if (> (`KismetArrayLibrary.Array_Length` _returnvalue_3) 0)
        (bind _item (`KismetArrayLibrary.Array_Get` _returnvalue_3))
        (bind _returnvalue_4 (`EnergyReceiverComponent.GetEnergy` _item "EnergyType_Corruption"))
        (`EnergyReceiverComponent.ModifyEnergy` _item "EnergyType_Corruption" (- (`KismetMathLibrary.FClamp` (+ _returnvalue_4 1000.0) 0.0 1800.0) _returnvalue_4)))
      (`/Game/Systems/Buffs/00_BP_AC_BuffSystem.AddBuff` (`self.GetComponentByClass` _array_element "/Game/Systems/Buffs/00_BP_AC_BuffSystem.00_BP_AC_BuffSystem_C") "/Game/Systems/Buffs/Damage_OverTime/BP_AC_Buff_Bleeding_WeaponProc.BP_AC_Buff_Bleeding_WeaponProc_C" null 1 null)))
  (`parent.ReceiveDestroyed`))

(fn `UserConstructionScript`
  (`parent.UserConstructionScript`))