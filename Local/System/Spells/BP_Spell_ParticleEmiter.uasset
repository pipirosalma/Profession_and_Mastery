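; Spell emitter actor that creates an area of Ymir's chilling effect around itself.
; On BeginPlay it reads the owning player's corruption energy and uses a sphere trace to destroy other nearby emitters of its class.
; Each tick it queries the player pawn registry and applies the chilling buff to nearby pawns with a buff system, sparing Ymir worshippers.
; Corruption scales both buff potency and the tick count before self-destruction.
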(event `self.ReceiveBeginPlay`
  (bind _returnvalue (`self.K2_GetActorLocation`))
  (bind _asbase_player_char (cast `/Game/Characters/BasePlayerChar` (`self.GetOwner`))
    (:`then`
      (set `self.Corruptionoftheowner` (`EnergyReceiverComponent.GetEnergy` (`/Game/Characters/BasePlayerChar.BPEnergyReceiver` _asbase_player_char) "EnergyType_Corruption")))
    (:`CastFailed`
      _))
  (`parent.ReceiveBeginPlay`)
  (bind _outhits (`KismetSystemLibrary.SphereTraceMulti` _returnvalue _returnvalue 500.0 "TraceTypeQuery1"))
  (for _array_element _outhits
    (bind _asbp_spell_particle_emiter (cast `/Local/System/Spells/BP_Spell_ParticleEmiter` (`.HitActor` (`GameplayStatics.BreakHitResult` _array_element))))
    (`self.K2_DestroyActor` _asbp_spell_particle_emiter)))

(event `self.ReceiveTick`
  (params (DeltaSeconds :type "Float (single-precision)"))
  (bind _controller (`/Game/Characters/FuncomFunctionLibrary.GetControllerFromActor` (`self.GetOwner`)))
  (bind _outactors (`GameplayStatics.GetAllActorsOfClass` "/Script/ConanSandbox.ConanWorldSettings"))
  (bind _returnvalue (`ConanWorldSettings.GetPlayerPawnRegistry` (`KismetArrayLibrary.Array_Get` _outactors)))
  (bind _returnvalue_2 (`PlayerPawnRegistry.GetPawnsWithinDistance` _returnvalue (`self.K2_GetActorLocation`) 500.0))
  (for _array_element _returnvalue_2
    (bind _returnvalue_3 (`self.K2_GetComponentsByClass` _array_element "/Game/Systems/Buffs/00_BP_AC_BuffSystem.00_BP_AC_BuffSystem_C"))
    (if (> (`KismetArrayLibrary.Array_Length` _returnvalue_3) 0)
      (bind _item (`KismetArrayLibrary.Array_Get` _returnvalue_3))
      (`self.NewMacro_0` _item
        (:`else`
          (`/Game/Systems/Buffs/00_BP_AC_BuffSystem.AddBuff` _item "/Game/Mods/Profession_and_Mastery/System/Spells/BP_AC_Buff_ChillingEffect_Ymir.BP_AC_Buff_ChillingEffect_Ymir_C" _controller (`KismetMathLibrary.FCeil` (* (/ (`self.Corruptionoftheowner`) 2000.0) 10.0)) _controller)))))
  (if (!= (`self.Corruptionoftheowner`) -1.0)
    (bind _result (`/Engine/EditorBlueprintResources/StandardMacros.IncrementFloat` (`self.Tick`))
      (:`  `
        (if (> _result (+ (* (/ (`self.Corruptionoftheowner`) 2000.0) 10.0) 2.0))
          (`self.K2_DestroyActor`))))))

(fn `UserConstructionScript`)