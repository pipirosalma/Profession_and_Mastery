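; Charm buff component that slows the owning character's movement and describes the reduction as a percentage.
; Buff potency sets the snare strength, scaled by the cripple modifier when the owner has the Encumberance_20 perk.
; The clamped speed multiplier is applied through the combat interface on start and removed on clear.
; Client start and clear events reuse that logic only off the server, preventing double application.
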(event `self.InitBuff`
  (params (DamageCauser :type "Actor Object Reference") (OwningCharacter :type "ConanCharacter Object Reference") (Instigator :type "Controller Object Reference"))
  (`parent.InitBuff` null OwningCharacter Instigator)
  (bind _asis_base_bpcombat_interface (cast `/Game/Systems/Interfaces/IsBaseBPCombatInterface` (`self.OwningCharacter`)))
  (set `self.ConbatInterface` _asis_base_bpcombat_interface))

(event `EffectToApplyOnBuffTick`)

(event `self.GameplayEffectToApplyOnBuffStart`
  (`parent.GameplayEffectToApplyOnBuffStart`)
  (set `self.SnareValue` (/ (`KismetMathLibrary.Conv_IntToDouble` (`self.BuffPotency`)) 10.0) :!label _label)
  (bind _asi_perk_system_owner_interface (cast `/Game/Systems/Perks/I_PerkSystemOwnerInterface` (`self.OwningCharacter`)))
  (bind _perksysteminterface (`/Game/Systems/Perks/I_PerkSystemOwnerInterface.GetPerkSystem` _asi_perk_system_owner_interface))
  (bind _hasperk (`/Game/Systems/Perks/I_PerkSystemInterface.HasPerk` _perksysteminterface "Encumberance_20"))
  (if _hasperk
    (bind _modifier (`/Game/Systems/Perks/I_PerkSystemInterface.GetPerksCrippleModifier` _perksysteminterface))
    (set `self.SnareValue` (* _modifier (`self.SnareValue`))))
  (bind _output_get (set `self.MovementSpeedMultiplier` (`KismetMathLibrary.FClamp` (- 1.0 (`self.SnareValue`)) 0.0 0.8)))
  (`/Game/Systems/Interfaces/IsBaseBPCombatInterface.AdjustMovementSpeedMultiplier` (`self.ConbatInterface`) true _output_get))

(event `self.ClientStartBuff`
  (params (OwningCharacter :type "ConanCharacter Object Reference") (Duration :type "Float (single-precision)"))
  (`parent.ClientStartBuff` OwningCharacter Duration)
  (bind _asis_base_bpcombat_interface (cast `/Game/Systems/Interfaces/IsBaseBPCombatInterface` (`self.OwningCharacter`)))
  (set `self.ConbatInterface` _asis_base_bpcombat_interface)
  ;[1 1 1] If we didn’t do this; then it would apply the effect twice
  (if (not (`KismetSystemLibrary.IsServer`))
    (goto _label)))

(event `self.GameplayEffectToApplyOnBuffCleared`
  (`parent.GameplayEffectToApplyOnBuffCleared`)
  (`/Game/Systems/Interfaces/IsBaseBPCombatInterface.AdjustMovementSpeedMultiplier` (`self.ConbatInterface`) false (`self.MovementSpeedMultiplier`) :!label _label_2)
  (set `self.MovementSpeedMultiplier` 0.0))

(event `self.ClientClearBuff`
  (params (OwningCharacter :type "ConanCharacter Object Reference"))
  (`parent.ClientClearBuff` OwningCharacter)
  ;[1 1 1] If we didn’t do this; then it would apply the effect twice
  (if (not (`KismetSystemLibrary.IsServer`))
    (goto _label_2)))

(fn `GetEffectDescription`
  (returns (Description :type Text))
  (return (`|FormatText` "Movement Speed reduced  by {SpeedModifier}%" (`KismetMathLibrary.Round` (* (- 1.0 (`self.MovementSpeedMultiplier`)) 100.0)))))