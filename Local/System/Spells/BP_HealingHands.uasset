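; Healing spell that puts a friendly bandage buff on another player character found by a sphere trace from the caster's head.
; After a 30-second delay it stops the tinkering montage and calls the parent use-item logic.
; A movement mode change on caster or target ends the buff and notifies of interruption.
; Lockpicking leftovers remain: door/chest difficulty, unlock roll and owner-online helpers go uncalled here, though skill level is still set.
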(event `SpellCastTrigger`
  (bind _asbase_player_char (cast `/Game/Characters/BasePlayerChar` (stale `self.OnUseItem` invokingCharacter) :!label _label))
  (bind _output_get (set `self.InvokingBasePlayer` _asbase_player_char))
  (`self.SetSkillLevel` _output_get)
  (bind _returnvalue (`Actor.GetComponentByClass` _output_get "/Script/Engine.SkeletalMeshComponent"))
  (bind _returnvalue_2 (`SceneComponent.GetSocketLocation` _returnvalue "b_head"))
  (bind _outhits (`KismetSystemLibrary.SphereTraceMulti` (+ _returnvalue_2 (0.0 0.0 10.0)) (- (+ (* (`SceneComponent.GetRightVector` _returnvalue) 160) _returnvalue_2) (0.0 0.0 130.0)) 20.0 "TraceTypeQuery1" false (`|MakeArray` (`Controller.K2_GetPawn` (`/Game/Characters/BasePlayerChar.PlayerController` _asbase_player_char)) :!type "Actor Object Reference")))
  (bind _asbase_player_char_2 (cast `/Game/Characters/BasePlayerChar` (`ActorComponent.GetOwner` (`.HitComponent` (`GameplayStatics.BreakHitResult` (`KismetArrayLibrary.Array_Get` _outhits)))))
    (:`then`
      (`/Game/Systems/Buffs/00_BP_AC_BuffSystem.AddBuff` (`/Game/Characters/BaseBPCombat.00_BP_AC_BuffSystem` _asbase_player_char_2) "/Game/Mods/Profession_and_Mastery/System/Spells/BP_AC_Buff_Bandage_Friendly.BP_AC_Buff_Bandage_Friendly_C" null 0 null)
      (add `Character.MovementModeChangedDelegate` _asbase_player_char_2 (delegate `EventLockpickEnd`))
      (add `Character.MovementModeChangedDelegate` (`self.InvokingBasePlayer`) (delegate `EventLockpickEnd`))
      (`KismetSystemLibrary.Delay` 30.0)
      (`/Game/Mods/Profession_and_Mastery/AC_Actor_Component_Main.AnimMontagePlay` (`Actor.GetComponentByClass` (`self.InvokingBasePlayer`) "/Game/Mods/Profession_and_Mastery/AC_Actor_Component_Main.AC_Actor_Component_Main_C") "/Game/Characters/humans/animations/emotes/AM_emote_tinkering.AM_emote_tinkering" false)
      (`parent.OnUseItem` (stale `self.OnUseItem` invokingCharacter) :!label _label_2))
    (:`CastFailed`
      (message `/Game/Characters/HUDNotification_Interface.NotificationText` (`/Game/Characters/FuncomFunctionLibrary.GetControllerFromActor` (`self.InvokingBasePlayer`)) "Couldn't find a valid target" false))))

(event `self.OnUseItem`
  (params (invokingCharacter :type "ConanCharacter Object Reference"))
  (goto _label))

(event `EventLockpickEnd`
  (params (Character :type "Character Object Reference") (PrevMovementMode :type "EMovementMode Enum") (PreviousCustomMode :type Byte))
  (`/Game/Systems/Buffs/00_BP_AC_BuffSystem.EndBuff` (`/Game/Characters/BaseBPCombat.00_BP_AC_BuffSystem` (stale `SpellCastTrigger` _asbase_player_char_2)) "/Game/Mods/Profession_and_Mastery/System/Spells/BP_AC_Buff_Bandage_Friendly.BP_AC_Buff_Bandage_Friendly_C")
  (`/Game/Mods/Profession_and_Mastery/AC_Actor_Component_Main.AnimMontagePlay` (`Actor.GetComponentByClass` (`self.InvokingBasePlayer`) "/Game/Mods/Profession_and_Mastery/AC_Actor_Component_Main.AC_Actor_Component_Main_C") "/Game/Characters/humans/animations/emotes/AM_emote_tinkering.AM_emote_tinkering" false)
  (message `/Game/Characters/HUDNotification_Interface.NotificationText` (`/Game/Characters/FuncomFunctionLibrary.GetControllerFromActor` (`self.InvokingBasePlayer`)) "Bandaging interrupted!" false)
  (goto _label_2))

(fn `CheckDifficulty`
  (params (Object :type "Object Object Reference"))
  (returns (`AsBP PL Door` :type "/Game/Systems/Building/Placeables/BP_PL_Door Object Reference") (`AsBP Master Placeables` :type "/Game/Systems/Building/Placeables/BP_Master_Placeables Object Reference") (False :type Boolean))
  (bind _asbp_pl_door (cast `/Game/Systems/Building/Placeables/BP_PL_Door` Object)
    (:`then`
      (set `self.IsDoor` true)
      (bind _output_get (set `self.DoorToOpen` _asbp_pl_door))
      (bind _returnvalue (`KismetSystemLibrary.GetDisplayName` _asbp_pl_door))
      (if (`KismetStringLibrary.Contains` _returnvalue "T1" false true)
        (set `self.LockDifficulty` 1)
        (elif (`KismetStringLibrary.Contains` _returnvalue "T2" false true)
          (set `self.LockDifficulty` 2)
          (elif (`KismetStringLibrary.Contains` _returnvalue "T3" false true)
            (set `self.LockDifficulty` 3)
            (else
              (return null null false)))))
      (return _output_get null true))
    (:`CastFailed`
      (bind _asbp_master_placeables (cast `/Game/Systems/Building/Placeables/BP_Master_Placeables` Object)
        (:`then`
          (set `self.ChestToUnlock` _asbp_master_placeables)
          (cast `/Game/Systems/Building/Placeables/BP_PL_Chest_Large` _asbp_master_placeables
            (:`then`
              (set `self.LockDifficulty` 2))
            (:`CastFailed`
              (cast `/Game/Systems/Building/Placeables/BP_PlaceableItemContainer` _asbp_master_placeables
                (:`then`
                  (set `self.LockDifficulty` 1))
                (:`CastFailed`
                  (set `self.LockDifficulty` 0)))))
          (return null _asbp_master_placeables true))
        (:`CastFailed`
          (set `self.LockDifficulty` 0)
          (return null null false))))))

(fn `CheckOwnerOnline`
  (params (BuildingPart :type "BuildableBase Object Reference"))
  (bind _returnvalue (`BuildableBase.GetOwnerName` BuildingPart))
  (set `self.ownername` (`KismetTextLibrary.Conv_TextToString` _returnvalue))
  (for _array_element (`/Game/Mods/Profession_and_Mastery/AC_Actor_Component_Main.ListOfOnlinePLayers` (`Actor.GetComponentByClass` (`self.InvokingBasePlayer`) "/Game/Mods/Profession_and_Mastery/AC_Actor_Component_Main.AC_Actor_Component_Main_C"))
    (bind _returnvalue_2 (`KismetStringLibrary.EqualEqual_StrStr` (`self.ownername`) _array_element))
    (if _returnvalue_2
      (set `self.OwnerOnline` _returnvalue_2)
      (else
        (`KismetSystemLibrary.PrintString` _array_element))))
  (return))