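; Buff spell that marks a player as watched by the god of a nearby altar.
; On start, a debug-drawn sphere trace from head bone down and rightward finds BP_PL_Altar hits and matches display names against GodList keys.
; Without a match the buff removes itself; otherwise it starts and swaps the "Prayer" widget for that god's icon and title.
; Tick events retry that update while the name remains "Prayer"; debug prints remain.
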(event `self.StartBuff`
  (params (BuffPotency :type Integer) (DamageCauser :type "Actor Object Reference") (OwningCharacter :type "ConanCharacter Object Reference") (Instigator :type "Controller Object Reference"))
  (bind _returnvalue (`Actor.GetComponentByClass` OwningCharacter "/Script/Engine.SkeletalMeshComponent"))
  (bind _returnvalue_2 (`SceneComponent.GetSocketLocation` _returnvalue "b_head"))
  (bind _asbase_player_char (cast `/Game/Characters/BasePlayerChar` OwningCharacter))
  (bind _outhits (`KismetSystemLibrary.SphereTraceMultiForObjects` (+ _returnvalue_2 (0.0 0.0 10.0)) (- (+ (* (`SceneComponent.GetRightVector` _returnvalue) 160) _returnvalue_2) (0.0 0.0 130.0)) 20.0 (`|MakeArray` "ObjectTypeQuery10" "ObjectTypeQuery2" :!type "EObjectTypeQuery Enum") false (`|MakeArray` (`Controller.K2_GetPawn` (`/Game/Characters/BasePlayerChar.PlayerController` _asbase_player_char)) :!type "Actor Object Reference") "ForDuration"))
  (for _array_element _outhits
    (bind _asbp_pl_altar (cast `/Game/Systems/Building/Placeables/BP_PL_Altar` (`self.GetOwner` (`.HitComponent` (`GameplayStatics.BreakHitResult` _array_element)))))
    (bind _keys (`BlueprintMapLibrary.Map_Keys` (`self.GodList`)))
    (for _array_element_2 _keys
      (bind _returnvalue_3 (`KismetSystemLibrary.GetDisplayName` _asbp_pl_altar))
      (`KismetSystemLibrary.PrintString` _returnvalue_3)
      (if (>= (`KismetStringLibrary.FindSubstring` _returnvalue_3 _array_element_2) 0)
        (set `self.WorshipedGod` _array_element_2))))
  (if (`KismetStringLibrary.NotEqual_StrStr` (`self.WorshipedGod`) "-1")
    (`self.UpdateClients`)
    (`parent.StartBuff` BuffPotency DamageCauser OwningCharacter Instigator)
    (else
      (`/Game/Systems/Buffs/00_BP_AC_BuffSystem.RemoveBuff` (`/Game/Characters/BaseBPCombat.00_BP_AC_BuffSystem` _asbase_player_char) "BP_Gods_Are_Watching_C"))))

(event `self.ClientDoBuffTick`
  (if (`KismetTextLibrary.EqualEqual_TextText` (`self.Name`) "Prayer") :!label _label
    (`self.UpdateClients`)))

(event `self.ReceiveTick`
  (params (DeltaSeconds :type "Float (single-precision)"))
  (goto _label))

(event `self.GameplayEffectToApplyOnBuffCleared`
  (`KismetSystemLibrary.PrintString` "Hello"))

(event `UpdateClients`
  (bind (_value _returnvalue) (`BlueprintMapLibrary.Map_Find` (`self.GodList`) (`self.WorshipedGod`)))
  (if (`KismetTextLibrary.EqualEqual_TextText` (`self.Name`) "Prayer")
    (`|ExecutionSequence`
      (:`then_0`
        (if (not (`KismetSystemLibrary.IsDedicatedServer`))
          (`self.RemoveBuffWidget`)))
      (:`then_1`
        (if _returnvalue
          (set `self.Icon` _value)
          (set `self.Name` (`KismetTextLibrary.Conv_StringToText` (`KismetStringLibrary.Concat_StrStr` (`self.WorshipedGod`) " is watching")))
          (`self.AddBuffWidget` (`self.BuffTickDuration`)))))))