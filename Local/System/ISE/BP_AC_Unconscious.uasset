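; Buff component that puts a player character into the Unconscious state for as long as the buff is active.
; On start it turns the state on through the owner's main actor component and binds to the character's state-change event.
; Any change to a state other than Unconscious re-applies it, so the state stays enforced.
; Clearing the buff unbinds the listener first, then turns the state off.
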(event `self.StartBuff`
  (params (BuffPotency :type Integer) (DamageCauser :type "Actor Object Reference") (OwningCharacter :type "ConanCharacter Object Reference") (Instigator :type "Controller Object Reference"))
  (`parent.StartBuff` BuffPotency DamageCauser OwningCharacter Instigator)
  (bind _asbase_player_char (cast `/Game/Characters/BasePlayerChar` OwningCharacter))
  (`/Game/Mods/Profession_and_Mastery/AC_Actor_Component_Main.HandleUnconsciousState` (`Actor.GetComponentByClass` _asbase_player_char "/Game/Mods/Profession_and_Mastery/AC_Actor_Component_Main.AC_Actor_Component_Main_C") true)
  (add `ConanCharacter.OnCharacterStateChanged` _asbase_player_char (delegate `EnforceUnconsciousState`)))

(event `self.ClearBuff`
  (`parent.ClearBuff`)
  (bind _asbase_player_char (cast `/Game/Characters/BasePlayerChar` (stale `self.StartBuff` OwningCharacter)))
  (remove `ConanCharacter.OnCharacterStateChanged` _asbase_player_char (delegate `EnforceUnconsciousState`))
  (`/Game/Mods/Profession_and_Mastery/AC_Actor_Component_Main.HandleUnconsciousState` (`Actor.GetComponentByClass` _asbase_player_char "/Game/Mods/Profession_and_Mastery/AC_Actor_Component_Main.AC_Actor_Component_Main_C") false))

(event `EnforceUnconsciousState`
  (params (OldState :type "ECharacterState Enum") (NewState :type "ECharacterState Enum"))
  (if (`|EnumInequality` NewState "Unconscious")
    (bind _asbase_player_char (cast `/Game/Characters/BasePlayerChar` (stale `self.StartBuff` OwningCharacter)))
    (`/Game/Mods/Profession_and_Mastery/AC_Actor_Component_Main.HandleUnconsciousState` (`Actor.GetComponentByClass` _asbase_player_char "/Game/Mods/Profession_and_Mastery/AC_Actor_Component_Main.AC_Actor_Component_Main_C") true)))