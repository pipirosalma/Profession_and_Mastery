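; Mod controller for a profession and class mastery mod that merges its custom feat, item, recipe, profession, stat, equipment and makeup color tables into the game's tables.
; On dedicated servers, every Tick rebuilds a list of online character and guild names from all player controllers and registers it with each pawn's AC_Actor_Component_Main.
; The looping timer meant to cache the owning player character is never started.
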(event `self.ReceiveBeginPlay`)

(event `WaitForValidPlayerController`
  (bind _asbase_player_char (cast `/Game/Characters/BasePlayerChar` (`self.GetOwner`)))
  (set `self.BasePlayerCharacter` _asbase_player_char)
  (`KismetSystemLibrary.K2_ClearAndInvalidateTimerHandle` (`self.LoopWaitTimer`)))

(event `self.ReceiveTick`
  (params (DeltaSeconds :type "Float (single-precision)"))
  (if (`KismetSystemLibrary.IsDedicatedServer`)
    (`KismetArrayLibrary.Array_Clear` (`self.ListOfOnlinePLayers`))
    (bind _outactors (`GameplayStatics.GetAllActorsOfClass` "/Game/Systems/FunCombat_PlayerController.FunCombat_PlayerController_C"))
    (for _array_element _outactors
      (`KismetArrayLibrary.Array_AddUnique` (`self.ListOfOnlinePLayers`) (`ConanPlayerController.GetCharacterName` _array_element))
      (bind _asbase_player_char (cast `/Game/Characters/BasePlayerChar` (`Controller.K2_GetPawn` _array_element)))
      (`KismetArrayLibrary.Array_AddUnique` (`self.ListOfOnlinePLayers`) (`Guild.GetGuildName` (`ConanCharacter.GetGuild` _asbase_player_char))))
    (for _array_element_2 _outactors
      (bind _asbase_player_char_2 (cast `/Game/Characters/BasePlayerChar` (`Controller.K2_GetPawn` _array_element_2)))
      (`/Game/Mods/Profession_and_Mastery/AC_Actor_Component_Main.RegisterPlayerList` (`self.GetComponentByClass` _asbase_player_char_2 "/Game/Mods/Profession_and_Mastery/AC_Actor_Component_Main.AC_Actor_Component_Main_C") (`self.ListOfOnlinePLayers`)))))

(fn `ModDataTableOperations`
  (`self.MergeDataTables` "/Game/Items/Feats/FeatTable.FeatTable" "/Game/Mods/Profession_and_Mastery/DataTables/dt_Feat_Table.dt_Feat_Table")
  (`self.MergeDataTables` "/Game/Items/ItemTable.ItemTable" "/Game/Mods/Profession_and_Mastery/DataTables/dt_Class_Mastery_Item_Table.dt_Class_Mastery_Item_Table")
  (`self.MergeDataTables` "/Game/Items/Recipes/RecipesTable.RecipesTable" "/Game/Mods/Profession_and_Mastery/DataTables/dt_Class_Mastery_Recipe_Table.dt_Class_Mastery_Recipe_Table")
  (`self.MergeDataTables` "/Game/Systems/SpawnTable/ProfessionTemplateDataTable.ProfessionTemplateDataTable" "/Game/Mods/Profession_and_Mastery/DataTables/dt_Profession_Template_Table.dt_Profession_Template_Table")
  (`self.MergeDataTables` "/Game/Items/ItemStatModificationTable.ItemStatModificationTable" "/Game/Mods/Profession_and_Mastery/DataTables/dt_custom_item_modif.dt_custom_item_modif")
  (`self.MergeDataTables` "/Game/Items/EquipmentVariationTable.EquipmentVariationTable" "/Game/Mods/Profession_and_Mastery/DataTables/dt_custom_equip_var.dt_custom_equip_var")
  (`self.MergeDataTables` "/Game/Items/ItemStatModificationTable.ItemStatModificationTable" "/Game/Mods/Profession_and_Mastery/DataTables/dt_OW_ItemStatModificationTable.dt_OW_ItemStatModificationTable")
  (`self.MergeDataTables` "/Game/UI/CharacterCreation/DataTables/EyeMakeupColorSelections.EyeMakeupColorSelections" "/Game/Mods/Profession_and_Mastery/DataTables/dt_corrupted_colours.dt_corrupted_colours")
  (`self.MergeDataTables` "/Game/UI/CharacterCreation/DataTables/LipMakeupColorSelections.LipMakeupColorSelections" "/Game/Mods/Profession_and_Mastery/DataTables/dt_corrupted_colours.dt_corrupted_colours")
  (`self.MergeDataTables` "/Game/Items/ItemStatModificationTable.ItemStatModificationTable" "/Game/Mods/Profession_and_Mastery/DataTables/dt_OW_DLC_ItemStatModificationTable.dt_OW_DLC_ItemStatModificationTable"))

(fn `UserConstructionScript`)

(fn `widget`)