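; AC_test is a test Blueprint that sketches adding a stylist icon panel to the character inventory's paperdoll UI, but none of its logic runs.
; BeginPlay, Tick and CraftingGUIActivated are empty.
; Disconnected nodes would bind to the CharacterInventory module's activation signal.
; Another orphaned chain waits briefly, finds visible W_PaperdollPanel widgets, and injects WStylistIconPanel two parents above the character display, setting IsPanelAdded.
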(event `Event CraftingGUIActivated`
  (params (module :type "GUIModule Object Reference") (isActive :type Boolean)))