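; Boots of The Explorer equippable item that grants the Agility_50 perk and changes footstep sounds for one specific player class.
; On equip it saves the wearer's footstep type, overrides it and adds the perk, then calls the parent logic.
; Unequip restores the saved footsteps, removes the perk and calls CheckAndApplyPerk to re-evaluate it.
; The Re-Run event re-adds the perk without checking class.
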(event `Re-Run`
  (params (Item :type "GameItem Object Reference"))
  (bind _asbase_player_char (cast `/Game/Characters/BasePlayerChar` (`self.OwnerActor`)))
  (`PerkSystemComponent.AddOwnedPerk` (`/Game/Characters/BasePlayerChar.BP_PerkSystemComponent` _asbase_player_char) "Agility_50"))

(event `self.OnEquip`
  (params (owner :type "Character Object Reference"))
  (bind _asbase_player_char (cast `/Game/Characters/BasePlayerChar` owner))
  (if (`|EnumEquality` (`/Game/Mods/Profession_and_Mastery/AC_Actor_Component_Main.PlayerClass` (`Actor.GetComponentByClass` _asbase_player_char "/Game/Mods/Profession_and_Mastery/AC_Actor_Component_Main.AC_Actor_Component_Main_C")) "NewEnumerator2")
    (bind _footsteptype (`/Game/Characters/BaseBPChar.GetFootstepSoundType` _asbase_player_char))
    (set `self.saved` _footsteptype)
    (set `/Game/Characters/BaseBPChar.FootstepType` "NewEnumerator18" _asbase_player_char)
    (`PerkSystemComponent.AddOwnedPerk` (`/Game/Characters/BasePlayerChar.BP_PerkSystemComponent` _asbase_player_char) "Agility_50"))
  (`parent.OnEquip` owner))

(event `self.OnUnEquip`
  (params (owner :type "Character Object Reference"))
  (bind _asbase_player_char (cast `/Game/Characters/BasePlayerChar` owner))
  (if (`|EnumEquality` (`/Game/Mods/Profession_and_Mastery/AC_Actor_Component_Main.PlayerClass` (`Actor.GetComponentByClass` _asbase_player_char "/Game/Mods/Profession_and_Mastery/AC_Actor_Component_Main.AC_Actor_Component_Main_C")) "NewEnumerator2")
    (set `/Game/Characters/BaseBPChar.FootstepType` (`self.saved`) _asbase_player_char)
    (bind _bp_perksystemcomponent (`/Game/Characters/BasePlayerChar.BP_PerkSystemComponent` _asbase_player_char))
    (`PerkSystemComponent.RemoveOwnedPerk` _bp_perksystemcomponent "Agility_50")
    (`/Game/Systems/Perks/BP_PerkSystemComponent.CheckAndApplyPerk` _bp_perksystemcomponent "Agility_50"))
  (`parent.OnUnEquip` owner))