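; Player controller component that lets a player change lip and eyeshadow color and pattern through the main radial menu.
; A top radial opens submenus filled from data table row names, with pattern tables chosen by sex.
; Each entry stores its row index in UserValue, which is written into the pawn's CharacterLayout before the submenu reopens after a delay.
; Tick holds leftover Return-entry tracking whose creation nodes are disconnected.
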(event `ChangeLipPattern`
  (params (LipPatternInt :type Integer))
  (bind _baseplayerchar (`self.GetBasePlayerChar`))
  (bind _characterlayout (`/Game/Characters/BasePlayerChar.CharacterLayout` _baseplayerchar))
  ;[1 1 1] Simple event to change hair int within CharacterLayout
  (setmembers `CharacterTextureLayout` :`StructRef` (`.TextureLayout` (break `CharacterLayout` _characterlayout)) :`LipTexture` LipPatternInt)
  (set `/Game/Characters/BasePlayerChar.CharacterLayout` _characterlayout _baseplayerchar))

(event `ChangeLipColor`
  (params (LipColorInt :type Integer))
  (bind _baseplayerchar (`self.GetBasePlayerChar`))
  (bind _characterlayout (`/Game/Characters/BasePlayerChar.CharacterLayout` _baseplayerchar))
  ;[1 1 1] Simple event to change hair int within CharacterLayout
  (setmembers `CharacterTintLayout` :`StructRef` (`.TintLayout` (break `CharacterLayout` _characterlayout)) :`LipMakeup` LipColorInt)
  (set `/Game/Characters/BasePlayerChar.CharacterLayout` _characterlayout _baseplayerchar))

(event `ShowMakeUpRadial`
  (bind _returnvalue (`GUIModuleController.GetGUIModuleController`))
  (bind _icontexture (`self.IconTexture`))
  ;[1 0.5506 0.1137] SHowMake-UpRadial
  (if (not (`GUIModuleController.IsModuleActive` _returnvalue "MainRadialMenu"))
    ;;[1 1 1] Activate or Deactivate if already activated
    (bind _returnvalue_2 (`GUIModuleController.ActivateModule` _returnvalue "MainRadialMenu" true false))
    (bind _asw_main_radial_menu (cast `/Game/UI/RadialMenus/W_MainRadialMenu` _returnvalue_2))
    (`|ExecutionSequence`
      (:`then_0`
        (bind _menu (`/Game/UI/RadialMenus/W_MainRadialMenu.Menu` _asw_main_radial_menu))
        ;;[1 1 1] Populate Radial Menu using index
        (bind _returnvalue_3 (`RadialMenu.AddItem` _menu (`|FormatText` "Lip Color") "" _icontexture "None" -1))
        (add `RadialMenuEntry.SignalClicked` _returnvalue_3 (delegate `OnMakeUpTypeSelected`)))
      (:`then_1`
        (bind _returnvalue_4 (`RadialMenu.AddItem` _menu (`|FormatText` "Lip Patternr") "" _icontexture "None" -1))
        (add `RadialMenuEntry.SignalClicked` _returnvalue_4 (delegate `OnMakeUpTypeSelect1`)))
      (:`then_2`
        (bind _returnvalue_5 (`RadialMenu.AddItem` _menu (`|FormatText` "Eye Shadow Color") "" _icontexture "None" -1))
        (add `RadialMenuEntry.SignalClicked` _returnvalue_5 (delegate `OnMakeUpTypeSelect2`)))
      (:`then_3`
        (bind _returnvalue_6 (`RadialMenu.AddItem` _menu (`|FormatText` "Eye Shadow Pattern") "" _icontexture "None" -1))
        (add `RadialMenuEntry.SignalClicked` _returnvalue_6 (delegate `OnMakeUpTypeSelect3`)))
      (:`then_4`
        ;;;[0.1707 1 0] Can't forget the Mr.Cancel Button XD
        (`RadialMenu.AddItem` _menu "Cancel" "" "/Game/UI/Textures/GUIs/MainRadialMenu/T_MainRadialMenuIconCancel.T_MainRadialMenuIconCancel" "None" -1)))
    (else
      (`GUIModuleController.ActivateModule` _returnvalue "MainRadialMenu" false false))))

(event `ShowLipColorRadial`
  (bind _returnvalue (`GUIModuleController.GetGUIModuleController`))
  (bind _isfemale (`self.GetIsFemale`))
  ;[1 0.5506 0.1137] ShowLipColorRadial
  (if (not (`GUIModuleController.IsModuleActive` _returnvalue "MainRadialMenu"))
    ;;[1 1 1] Activate or Deactivate if already activated
    (bind _returnvalue_2 (`GUIModuleController.ActivateModule` _returnvalue "MainRadialMenu" true false))
    (bind _asw_main_radial_menu (cast `/Game/UI/RadialMenus/W_MainRadialMenu` _returnvalue_2))
    (if _isfemale
      (bind _outrownames (`DataTableFunctionLibrary.GetDataTableRowNames` "/Game/UI/CharacterCreation/DataTables/LipMakeupColorSelections.LipMakeupColorSelections"))
      (for (_array_element _array_index) _outrownames
        (bind _menu (`/Game/UI/RadialMenus/W_MainRadialMenu.Menu` _asw_main_radial_menu))
        ;;[1 1 1] Populate Radial Menu using index
        (bind _returnvalue_3 (`RadialMenu.AddItem` _menu (`|FormatText` "LipColor {index}" (`KismetTextLibrary.Conv_NameToText` (select `bool` _isfemale :`false` (stale _array_element_2) :`true` _array_element))) "A stunning color" (`self.IconTexture`) "None" -1 :!label _label))
        ;;;[1 1 1] Sneaky
        (set `RadialMenuEntry.UserValue` (select `bool` _isfemale :`false` (stale _array_index_2) :`true` _array_index) _returnvalue_3)
        (add `RadialMenuEntry.SignalClicked` _returnvalue_3 (delegate `OnLipColorSelected`)))
      (else
        (bind _outrownames_2 (`DataTableFunctionLibrary.GetDataTableRowNames` "/Game/UI/CharacterCreation/DataTables/LipMakeupColorSelections.LipMakeupColorSelections"))
        (for (_array_element_2 _array_index_2) _outrownames_2
          (goto _label))))
    ;;[0.1707 1 0] Can't forget the Mr.Cancel Button XD
    (`RadialMenu.AddItem` _menu "Cancel" "" "/Game/UI/Textures/GUIs/MainRadialMenu/T_MainRadialMenuIconCancel.T_MainRadialMenuIconCancel" "None" -1)
    (bind _returnvalue_4 (`RadialMenu.AddItem` _menu "Return" " " "/Game/UI/Textures/GUIs/ExilesJourney/icon_exilesJourney_unlocked.icon_exilesJourney_unlocked" "None" -1))
    (add `RadialMenuEntry.SignalClicked` _returnvalue_4 (delegate `CustomEvent_2`))
    (else
      (`GUIModuleController.ActivateModule` _returnvalue "MainRadialMenu" false false))))

(event `ShowLipPatternRadial`
  (bind _returnvalue (`GUIModuleController.GetGUIModuleController`))
  (bind _isfemale (`self.GetIsFemale`))
  ;[1 0.5506 0.1137] ShowLipPatternRadial
  (if (not (`GUIModuleController.IsModuleActive` _returnvalue "MainRadialMenu"))
    ;;[1 1 1] Activate or Deactivate if already activated
    (bind _returnvalue_2 (`GUIModuleController.ActivateModule` _returnvalue "MainRadialMenu" true false))
    (bind _asw_main_radial_menu (cast `/Game/UI/RadialMenus/W_MainRadialMenu` _returnvalue_2))
    (if _isfemale
      (bind _outrownames (`DataTableFunctionLibrary.GetDataTableRowNames` "/Game/UI/CharacterCreation/DataTables/Female_LipsSelections.Female_LipsSelections"))
      (for (_array_element _array_index) _outrownames
        (bind _menu (`/Game/UI/RadialMenus/W_MainRadialMenu.Menu` _asw_main_radial_menu))
        ;;[1 1 1] Populate Radial Menu using index
        (bind _returnvalue_3 (`RadialMenu.AddItem` _menu (`|FormatText` "Lipstick Pattern {index}" (`KismetTextLibrary.Conv_NameToText` (select `bool` _isfemale :`false` (stale _array_element_2) :`true` _array_element))) "A stunning Lipstick Pattern" (`self.IconTexture`) "None" -1 :!label _label_2))
        ;;;[1 1 1] Sneaky
        (set `RadialMenuEntry.UserValue` (select `bool` _isfemale :`false` (stale _array_index_2) :`true` _array_index) _returnvalue_3)
        (add `RadialMenuEntry.SignalClicked` _returnvalue_3 (delegate `OnLipPatternSelected`)))
      (else
        (bind _outrownames_2 (`DataTableFunctionLibrary.GetDataTableRowNames` "/Game/UI/CharacterCreation/DataTables/Male_LipsSelections.Male_LipsSelections"))
        (for (_array_element_2 _array_index_2) _outrownames_2
          (goto _label_2))))
    ;;[0.1707 1 0] Can't forget the Mr.Cancel Button XD
    (`RadialMenu.AddItem` _menu "Cancel" "" "/Game/UI/Textures/GUIs/MainRadialMenu/T_MainRadialMenuIconCancel.T_MainRadialMenuIconCancel" "None" -1)
    (bind _returnvalue_4 (`RadialMenu.AddItem` _menu "Return" " " "/Game/UI/Textures/GUIs/ExilesJourney/icon_exilesJourney_unlocked.icon_exilesJourney_unlocked" "None" -1))
    (add `RadialMenuEntry.SignalClicked` _returnvalue_4 (delegate `CustomEvent_1`))
    (else
      (`GUIModuleController.ActivateModule` _returnvalue "MainRadialMenu" false false))))

(event `OnMakeUpTypeSelected`
  (params (menuEntry :type "RadialMenuEntry Object Reference"))
  ;[1 0.5506 0.1137] SHowMake-UpRadial
  (`KismetSystemLibrary.Delay` 0.2)
  (`self.ShowLipColorRadial`))

(event `OnLipColorSelected`
  (params (menuEntry :type "RadialMenuEntry Object Reference"))
  ;[1 0.5506 0.1137] ShowLipColorRadial
  (`self.ChangeLipColor` (`RadialMenuEntry.UserValue` menuEntry))
  (`KismetSystemLibrary.Delay` 2.0)
  (`self.ShowLipColorRadial`))

(event `OnLipPatternSelected`
  (params (menuEntry :type "RadialMenuEntry Object Reference"))
  ;[1 0.5506 0.1137] ShowLipPatternRadial
  (`self.ChangeLipPattern` (`RadialMenuEntry.UserValue` menuEntry))
  (`KismetSystemLibrary.Delay` 2.0)
  (`self.ShowLipPatternRadial`))

(event `OnMakeUpTypeSelect1`
  (params (menuEntry :type "RadialMenuEntry Object Reference"))
  ;[1 0.5506 0.1137] SHowMake-UpRadial
  (`KismetSystemLibrary.Delay` 0.2)
  (`self.ShowLipPatternRadial`))

(event `OnMakeUpTypeSelect2`
  (params (menuEntry :type "RadialMenuEntry Object Reference"))
  ;[1 0.5506 0.1137] SHowMake-UpRadial
  (`KismetSystemLibrary.Delay` 0.2)
  (`self.SHowEyeShadowColorRadial`))

(event `CustomEvent_1`
  (params (menuEntry :type "RadialMenuEntry Object Reference"))
  (`KismetSystemLibrary.Delay` 0.2)
  (`self.ShowMakeUpRadial`))

(event `ChangeEyeshadowColor`
  (params (EyeShadowInt :type Integer))
  (bind _baseplayerchar (`self.GetBasePlayerChar`))
  (bind _characterlayout (`/Game/Characters/BasePlayerChar.CharacterLayout` _baseplayerchar))
  (setmembers `CharacterTintLayout` :`StructRef` (`.TintLayout` (break `CharacterLayout` _characterlayout)) :`EyeMakeup` EyeShadowInt)
  (set `/Game/Characters/BasePlayerChar.CharacterLayout` _characterlayout _baseplayerchar))

(event `CustomEvent_2`
  (params (menuEntry :type "RadialMenuEntry Object Reference"))
  (`KismetSystemLibrary.Delay` 0.2)
  (`self.ShowMakeUpRadial`))

(event `ChangeEyeShadowPattern`
  (params (EyeShadowPatternInt :type Integer))
  (bind _baseplayerchar (`self.GetBasePlayerChar`))
  (bind _characterlayout (`/Game/Characters/BasePlayerChar.CharacterLayout` _baseplayerchar))
  ;[1 1 1] Simple event to change hair int within CharacterLayout
  (setmembers `CharacterTextureLayout` :`StructRef` (`.TextureLayout` (break `CharacterLayout` _characterlayout)) :`EyeTexture` EyeShadowPatternInt)
  (set `/Game/Characters/BasePlayerChar.CharacterLayout` _characterlayout _baseplayerchar))

(event `OnMakeUpTypeSelect3`
  (params (menuEntry :type "RadialMenuEntry Object Reference"))
  ;[1 0.5506 0.1137] SHowMake-UpRadial
  (`KismetSystemLibrary.Delay` 0.2)
  (`self.ShowEyeShadowPatternRadial`))

(event `SHowEyeShadowColorRadial`
  (bind _returnvalue (`GUIModuleController.GetGUIModuleController`))
  (bind _isfemale (`self.GetIsFemale`))
  ;[1 0.5506 0.1137] ShowEyeShadowColorRadial
  (if (not (`GUIModuleController.IsModuleActive` _returnvalue "MainRadialMenu"))
    ;;[1 1 1] Activate or Deactivate if already activated
    (bind _returnvalue_2 (`GUIModuleController.ActivateModule` _returnvalue "MainRadialMenu" true false))
    (bind _asw_main_radial_menu (cast `/Game/UI/RadialMenus/W_MainRadialMenu` _returnvalue_2))
    (if _isfemale
      (bind _outrownames (`DataTableFunctionLibrary.GetDataTableRowNames` "/Game/UI/CharacterCreation/DataTables/EyeMakeupColorSelections.EyeMakeupColorSelections"))
      (for (_array_element _array_index) _outrownames
        (bind _menu (`/Game/UI/RadialMenus/W_MainRadialMenu.Menu` _asw_main_radial_menu))
        ;;[1 1 1] Populate Radial Menu using index
        (bind _returnvalue_3 (`RadialMenu.AddItem` _menu (`|FormatText` "Eyeshadow Color {index}" (`KismetTextLibrary.Conv_NameToText` (select `bool` _isfemale :`false` (stale _array_element_2) :`true` _array_element))) "A stunning Eyeshadow Color" (`self.IconTexture`) "None" -1 :!label _label_3))
        ;;;[1 1 1] Sneaky
        (set `RadialMenuEntry.UserValue` (select `bool` _isfemale :`false` (stale _array_index_2) :`true` _array_index) _returnvalue_3)
        (add `RadialMenuEntry.SignalClicked` _returnvalue_3 (delegate `OnOnEyeShadowColorSelected`)))
      (else
        (bind _outrownames_2 (`DataTableFunctionLibrary.GetDataTableRowNames` "/Game/UI/CharacterCreation/DataTables/EyeMakeupColorSelections.EyeMakeupColorSelections"))
        (for (_array_element_2 _array_index_2) _outrownames_2
          (goto _label_3))))
    ;;[0.1707 1 0] Can't forget the Mr.Cancel Button XD
    (`RadialMenu.AddItem` _menu "Cancel" "" "/Game/UI/Textures/GUIs/MainRadialMenu/T_MainRadialMenuIconCancel.T_MainRadialMenuIconCancel" "None" -1)
    (bind _returnvalue_4 (`RadialMenu.AddItem` _menu "Return" " " "/Game/UI/Textures/GUIs/ExilesJourney/icon_exilesJourney_unlocked.icon_exilesJourney_unlocked" "None" -1))
    (add `RadialMenuEntry.SignalClicked` _returnvalue_4 (delegate `Unlock_SignalClicked`))
    (else
      (`GUIModuleController.ActivateModule` _returnvalue "MainRadialMenu" false false))))

(event `ShowEyeShadowPatternRadial`
  (bind _returnvalue (`GUIModuleController.GetGUIModuleController`))
  (bind _isfemale (`self.GetIsFemale`))
  ;[1 0.5506 0.1137] ShowEyeShadowPatternRadial
  (if (not (`GUIModuleController.IsModuleActive` _returnvalue "MainRadialMenu"))
    ;;[1 1 1] Activate or Deactivate if already activated
    (bind _returnvalue_2 (`GUIModuleController.ActivateModule` _returnvalue "MainRadialMenu" true false))
    (bind _asw_main_radial_menu (cast `/Game/UI/RadialMenus/W_MainRadialMenu` _returnvalue_2))
    (if _isfemale
      (bind _outrownames (`DataTableFunctionLibrary.GetDataTableRowNames` "/Game/UI/CharacterCreation/DataTables/Female_EyesSelections.Female_EyesSelections"))
      (for (_array_element _array_index) _outrownames
        (bind _menu (`/Game/UI/RadialMenus/W_MainRadialMenu.Menu` _asw_main_radial_menu))
        ;;[1 1 1] Populate Radial Menu using index
        (bind _returnvalue_3 (`RadialMenu.AddItem` _menu (`|FormatText` "Eye Shadow Pattern {index}" (`KismetTextLibrary.Conv_NameToText` (select `bool` _isfemale :`false` (stale _array_element_2) :`true` _array_element))) "A stunning Eyeshadow Pattern" (`self.IconTexture`) "None" -1 :!label _label_4))
        ;;;[1 1 1] Sneaky
        (set `RadialMenuEntry.UserValue` (select `bool` _isfemale :`false` (stale _array_index_2) :`true` _array_index) _returnvalue_3)
        (add `RadialMenuEntry.SignalClicked` _returnvalue_3 (delegate `OnEyeShadowPatternSelected`)))
      (else
        (bind _outrownames_2 (`DataTableFunctionLibrary.GetDataTableRowNames` "/Game/UI/CharacterCreation/DataTables/Male_EyesSelections.Male_EyesSelections"))
        (for (_array_element_2 _array_index_2) _outrownames_2
          (goto _label_4))))
    ;;[0.1707 1 0] Can't forget the Mr.Cancel Button XD
    (`RadialMenu.AddItem` _menu "Cancel" "" "/Game/UI/Textures/GUIs/MainRadialMenu/T_MainRadialMenuIconCancel.T_MainRadialMenuIconCancel" "None" -1)
    (bind _returnvalue_4 (`RadialMenu.AddItem` _menu "Return" " " "/Game/UI/Textures/GUIs/ExilesJourney/icon_exilesJourney_unlocked.icon_exilesJourney_unlocked" "None" -1))
    (add `RadialMenuEntry.SignalClicked` _returnvalue_4 (delegate `CustomEvent`))
    (else
      (`GUIModuleController.ActivateModule` _returnvalue "MainRadialMenu" false false))))

(event `OnOnEyeShadowColorSelected`
  (params (menuEntry :type "RadialMenuEntry Object Reference"))
  ;[1 0.5506 0.1137] ShowEyeShadowColorRadial
  (`self.ChangeEyeshadowColor` (`RadialMenuEntry.UserValue` menuEntry))
  (`KismetSystemLibrary.Delay` 2.0)
  (`self.SHowEyeShadowColorRadial`))

(event `OnEyeShadowPatternSelected`
  (params (menuEntry :type "RadialMenuEntry Object Reference"))
  ;[1 0.5506 0.1137] ShowEyeShadowPatternRadial
  (`self.ChangeEyeShadowPattern` (`RadialMenuEntry.UserValue` menuEntry))
  (`KismetSystemLibrary.Delay` 2.0)
  (`self.ShowEyeShadowPatternRadial`))

(event `Unlock_SignalClicked`
  (params (menuEntry :type "RadialMenuEntry Object Reference"))
  (`KismetSystemLibrary.Delay` 0.2)
  (`self.ShowMakeUpRadial`))

(event `CustomEvent`
  (params (menuEntry :type "RadialMenuEntry Object Reference"))
  (`KismetSystemLibrary.Delay` 0.2)
  (`self.ShowMakeUpRadial`))

(event `self.ReceiveTick`
  (params (DeltaSeconds :type "Float (single-precision)"))
  (bind _returnvalue (`GUIModuleController.GetGUIModuleController`))
  ;[1 1 1] Is RadialMenu active?
  (if (`GUIModuleController.IsModuleActive` _returnvalue "MainRadialMenu")
    ;[1 1 1] This will do for now :/
    (bind _returnvalue_2 (`GUIModuleController.ActivateModule` _returnvalue "MainRadialMenu" true false))
    (bind _asw_main_radial_menu (cast `/Game/UI/RadialMenus/W_MainRadialMenu` _returnvalue_2))
    ;[1 1 1] Is already added?
    (if (`KismetSystemLibrary.IsValid` (`self.radialSeg`))
      _)
    (else
      ;[1 1 1] If RadialMenu is not active, and radialSeg is still referenced set to NULL
      (if (`KismetSystemLibrary.IsValid` (`self.radialSeg`))
        (set `self.radialSeg` null)))))

(event `CustomEvent_3`
  (params (menuEntry :type "RadialMenuEntry Object Reference")))

(fn `GetBasePlayerChar`
  (returns (BasePlayerChar :type "/Game/Characters/BasePlayerChar Object Reference"))
  (bind _asfun_combat_player_controller (cast `/Game/Systems/FunCombat_PlayerController` (`self.GetOwner`))
    (:`then`
      (bind _asbase_player_char (cast `/Game/Characters/BasePlayerChar` (`Controller.K2_GetPawn` _asfun_combat_player_controller))
        (:`then`
          _)
        (:`CastFailed`
          _)))
    (:`CastFailed`
      _))
  (return _asbase_player_char))

(fn `GetIsFemale`
  (returns (isFemale :type Boolean))
  (return (break `CharacterBoolParameters` (`.BoolParams` (break `CharacterLayout` (`/Game/Characters/BasePlayerChar.CharacterLayout` (`self.GetBasePlayerChar`)))))))