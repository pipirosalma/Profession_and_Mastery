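; Player character component that tracks drug and alcohol addiction and applies a withdrawal debuff.
; It listens to the buff system: drunkenness and drug buffs raise the addiction level by different amounts, reset the last-high timer and clear withdrawal.
; Each tick decays the level, removing withdrawal below the threshold.
; Otherwise, withdrawal starts after a sober delay that shortens as addiction grows, with potency scaled to the level.
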(event `self.ReceiveBeginPlay`
  (bind _asbase_player_char (cast `/Game/Characters/BasePlayerChar` (`self.GetOwner`)))
  (add `/Game/Systems/Buffs/00_BP_AC_BuffSystem.SignalBuffAdded` (`/Game/Characters/BaseBPCombat.00_BP_AC_BuffSystem` _asbase_player_char) (delegate `RegisterBuff`)))

(event `RegisterBuff`
  (params (buff :type "/Game/Systems/Buffs/01_BP_AC_Buff_Master Object Reference"))
  (cast `/Game/Systems/Buffs/Alcohol/BP_AC_Buff_Drunkenness` buff
    (:`then`
      (set `self.Addiction Level` (+ (`self.Addiction Level`) 0.1))
      (set `self.LastTimeHigh` (`GameplayStatics.GetTimeSeconds`))
      (bind _00_bp_ac_buffsystem (`/Game/Characters/BaseBPCombat.00_BP_AC_BuffSystem` (stale `self.ReceiveBeginPlay` _asbase_player_char)))
      (`/Game/Systems/Buffs/00_BP_AC_BuffSystem.RemoveBuff` _00_bp_ac_buffsystem "/Game/Mods/Profession_and_Mastery/System/Buffs/BP_Debuff_Withdraw.BP_Debuff_Withdraw_C"))
    (:`CastFailed`
      (cast `/Game/Mods/Profession_and_Mastery/System/Buffs/BP_Drugs_Master` buff)
      (set `self.Addiction Level` (+ (`self.Addiction Level`) 0.3))
      (set `self.LastTimeHigh` (`GameplayStatics.GetTimeSeconds`))
      (`/Game/Systems/Buffs/00_BP_AC_BuffSystem.RemoveBuff` _00_bp_ac_buffsystem "/Game/Mods/Profession_and_Mastery/System/Buffs/BP_Debuff_Withdraw.BP_Debuff_Withdraw_C"))))

(event `self.ReceiveTick`
  (params (DeltaSeconds :type "Float (single-precision)"))
  (bind _addiction_level (`self.Addiction Level`))
  (bind _returnvalue (> 1.0 (`self.Addiction Level`)))
  (if (> _addiction_level 0.0)
    (set `self.Addiction Level` (- _addiction_level 0.1))
    (elif (> 0.0 _addiction_level)
      (set `self.Addiction Level` 0.0)))
  (bind _asbase_player_char (cast `/Game/Characters/BasePlayerChar` (`self.GetOwner`)))
  (if _returnvalue
    (bind _00_bp_ac_buffsystem (`/Game/Characters/BaseBPCombat.00_BP_AC_BuffSystem` _asbase_player_char))
    (bind _hasbuff (`/Game/Systems/Buffs/00_BP_AC_BuffSystem.CheckIfBuffExists` _00_bp_ac_buffsystem "/Game/Mods/Profession_and_Mastery/System/Buffs/BP_Debuff_Withdraw.BP_Debuff_Withdraw_C"))
    (if _hasbuff
      (`/Game/Systems/Buffs/00_BP_AC_BuffSystem.RemoveBuff` _00_bp_ac_buffsystem "/Game/Mods/Profession_and_Mastery/System/Buffs/BP_Debuff_Withdraw.BP_Debuff_Withdraw_C"))
    (else
      (`/Game/Systems/BP_MacroGlobal.And+Branch` (not _returnvalue) (not _hasbuff)
        (:`True`
          (if (>= (- (`GameplayStatics.GetTimeSeconds`) (`self.LastTimeHigh`)) (- 600.0 (* (`self.Addiction Level`) 10.0)))
            (`/Game/Systems/Buffs/00_BP_AC_BuffSystem.AddBuff` _00_bp_ac_buffsystem "/Game/Mods/Profession_and_Mastery/System/Buffs/BP_Debuff_Withdraw.BP_Debuff_Withdraw_C" null (`KismetMathLibrary.FFloor` (`self.Addiction Level`)) null)))))))