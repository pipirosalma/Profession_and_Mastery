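; Thrown knife weapon Blueprint that handles visibility and ammo consumption when the knife is thrown.
; Throwing hides the visual actor, and ending the attack shows it again.
; For player or non-ConanCharacter owners, each throw lowers the replicated StackSize, setting -1 on the last knife and force-unequipping on the server; non-player ConanCharacters keep their stack.
; Projectiles report the weapon's TemplateID as their launcher.
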(fn `GetLauncherTemplateId`
  (params (Projectile :type "/Game/Items/Weapons/BP_BaseProjectile Object Reference") (Weapon :type "/Game/Items/BPGameItemWeapon Object Reference"))
  (returns (PickableAmmoTemplateId :type Integer))
  (return (`GameItem.TemplateID` Weapon)))

(fn `WeaponAttackEnd`
  (returns (Success :type Boolean))
  (`Actor.SetActorHiddenInGame` (`self.VisualActor`) false)
  (return true))

(fn `WeaponThrown`
  (returns (Success :type Boolean))
  (bind _returnvalue (`self.GetIntStat` "StackSize"))
  (`Actor.SetActorHiddenInGame` (`self.VisualActor`) true)
  (bind _asconan_character (cast `ConanCharacter` (`self.GetOwner`))
    (:`then`
      (if (`ConanCharacter.IsPlayer` _asconan_character)
        (if (< _returnvalue 2) :!label _label
          (`self.SetIntStat` "StackSize" -1)
          (else
            (`self.SetIntStat` "StackSize" (- _returnvalue 1))))
        (`/Game/Systems/BP_MacroGlobal.And+Branch` (< (`self.GetIntStat` "StackSize") 1) (`KismetSystemLibrary.IsServer`)
          (:`True`
            (`self.ForceUnequip`))
          (:`False`
            _))))
    (:`CastFailed`
      (goto _label)))
  (return true))