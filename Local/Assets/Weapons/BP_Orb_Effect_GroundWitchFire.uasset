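; Witchfire ground area effect for an orb weapon that burns and debuffs combat characters inside its sphere.
; The server runs a looping timer that applies radial health and explosive damage, the latter scaled by fade delay.
; Overlaps add the Witchfire buff and track affected characters.
; Setting HasExploded triggers client-only particle collision binding, moving and activating secondary fire particles at impacts near the sphere.
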(event `ParticleStart`
  (if (not (`KismetSystemLibrary.IsServer`))
    (`self.Orb_Fire_Collide` "None")))

(event `Orb_Fire_Collide`
  (params (EventName :type Name) (EmitterTime :type "Float (double-precision)") (ParticleTime :type Integer) (Location :type "Vector Structure") (Velocity :type "Vector Structure") (Direction :type "Vector Structure") (Normal :type "Vector Structure") (BoneName :type Name) (PhysMat :type "PhysicalMaterial Object Reference"))
  (bind _particlesystem2 (`self.ParticleSystem2`))
  (if (not (`KismetSystemLibrary.IsServer`))
    (add `ParticleSystemComponent.OnParticleCollide` (`self.ParticleSystem`) (delegate `Orb_Fire_Collide`))
    (if (< (`KismetMathLibrary.VSize` (- Location (`self.K2_GetActorLocation`))) (* (`SphereComponent.SphereRadius` (`self.Sphere`)) 1.5))
      (`SceneComponent.K2_SetWorldLocation` _particlesystem2 Location false false)
      (`SceneComponent.K2_SetWorldLocation` (`self.ParticleSystem3`) Location false false)
      (`ActorComponent.Activate` _particlesystem2 false)
      (`ActorComponent.Activate` (`self.ParticleSystem3`) false))))

(event `self.ReceiveBeginPlay`
  (`parent.ReceiveBeginPlay`)
  (set `self.HasExploded` true)
  (if (`KismetSystemLibrary.IsServer`)
    (`KismetSystemLibrary.K2_SetTimerDelegate` (delegate `DoDamage`) 0.5 true)))

(event `self.Sphere.OnComponentBeginOverlap`
  (params (OverlappedComponent :type "PrimitiveComponent Object Reference") (OtherActor :type "Actor Object Reference") (OtherComp :type "PrimitiveComponent Object Reference") (OtherBodyIndex :type Integer) (bFromSweep :type Boolean) (SweepResult :type "HitResult Structure (by ref)"))
  (bind _asbase_bpcombat (cast `/Game/Characters/BaseBPCombat` OtherActor))
  (`KismetArrayLibrary.Array_Add` (`self.BuffAffectedChars`) _asbase_bpcombat)
  (`/Game/Systems/Buffs/00_BP_AC_BuffSystem.AddBuff` (`/Game/Characters/BaseBPCombat.00_BP_AC_BuffSystem` _asbase_bpcombat) "/Game/Mods/Profession_and_Mastery/Assets/Weapons/BP_AC_Buff_Witchfire.BP_AC_Buff_Witchfire_C" self 0 (`/Game/Characters/FuncomFunctionLibrary.GetControllerFromActor` (`self.Instigator`))))

(event `DoDamage`
  (bind _returnvalue (`self.K2_GetActorLocation`))
  (bind _returnvalue_2 (`Pawn.GetController` (`self.Instigator`)))
  (bind _sphereradius (`SphereComponent.SphereRadius` (`self.Sphere`)))
  (`ApplyRadialDamageWithFalloffProxy.ApplyRadialDamageAsync` :`BaseDamage` 10.0 :`Origin` _returnvalue :`DamageRadius` _sphereradius :`DamageTypeClass` "/Game/Systems/Progression/DmgTypeHealth_BP.DmgTypeHealth_BP_C" :`DamageCauser` self :`InstigatedByController` _returnvalue_2 :`bDoFullDamage` true
    (:`then`
      (`ApplyRadialDamageWithFalloffProxy.ApplyRadialDamageAsync` :`BaseDamage` (/ 500.0 (`self.DelayUntilFadeEffects`)) :`Origin` _returnvalue :`DamageRadius` _sphereradius :`DamageTypeClass` "/Game/Systems/Combat/Dmg_Explosive.Dmg_Explosive_C" :`DamageCauser` self :`InstigatedByController` _returnvalue_2 :`bDoFullDamage` true))))

(event `self.Sphere.OnComponentEndOverlap`
  (params (OverlappedComponent :type "PrimitiveComponent Object Reference") (OtherActor :type "Actor Object Reference") (OtherComp :type "PrimitiveComponent Object Reference") (OtherBodyIndex :type Integer))
  (bind _asbase_bpcombat (cast `/Game/Characters/BaseBPCombat` OtherActor))
  (`KismetArrayLibrary.Array_RemoveItem` (`self.BuffAffectedChars`) _asbase_bpcombat))

(fn `OnRep_HasExploded`
  (`self.ParticleStart`))

(fn `UserConstructionScript`
  (`parent.UserConstructionScript`))