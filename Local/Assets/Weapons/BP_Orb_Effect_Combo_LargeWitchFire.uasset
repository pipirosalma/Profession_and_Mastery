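; Area effect for the large witchfire orb combo, dealing periodic damage and applying the Witchfire buff to combat characters who enter it.
; On the server, a looping timer applies asynchronous radial health and explosive damage if PvP is allowed or an instigator is valid.
; Explosive damage scales inversely with fade delay, and the sphere's radius sets the damage radius.
; Sphere overlaps add the buff and track affected characters; leaving only untracks them.
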(event `self.ReceiveBeginPlay`
  (`parent.ReceiveBeginPlay`)
  (if (`KismetSystemLibrary.IsServer`)
    (`KismetSystemLibrary.K2_SetTimerDelegate` (delegate `DoDamage`) 0.5 true)))

(event `DoDamage`
  (bind _returnvalue (`self.K2_GetActorLocation`))
  (bind _damageradius (`self.DamageRadius`))
  (bind _returnvalue_2 (`Pawn.GetController` (`self.Instigator`)))
  (bind _asconan_game_state (cast `ConanGameState` (`GameplayStatics.GetGameState`)))
  (if (or (`ConanGameState.IsPVPAllowed` _asconan_game_state) (`KismetSystemLibrary.IsValid` (`self.Instigator`)))
    (`ApplyRadialDamageWithFalloffProxy.ApplyRadialDamageAsync` :`BaseDamage` 10.0 :`Origin` _returnvalue :`DamageRadius` _damageradius :`DamageTypeClass` "/Game/Systems/Progression/DmgTypeHealth_BP.DmgTypeHealth_BP_C" :`DamageCauser` self :`InstigatedByController` _returnvalue_2 :`bDoFullDamage` true
      (:`then`
        (`ApplyRadialDamageWithFalloffProxy.ApplyRadialDamageAsync` :`BaseDamage` (/ 500.0 (`self.DelayUntilFadeEffects`)) :`Origin` _returnvalue :`DamageRadius` _damageradius :`DamageTypeClass` "/Game/Systems/Combat/Dmg_Explosive.Dmg_Explosive_C" :`DamageCauser` self :`InstigatedByController` _returnvalue_2 :`bDoFullDamage` true)))))

(event `self.Sphere.OnComponentBeginOverlap`
  (params (OverlappedComponent :type "PrimitiveComponent Object Reference") (OtherActor :type "Actor Object Reference") (OtherComp :type "PrimitiveComponent Object Reference") (OtherBodyIndex :type Integer) (bFromSweep :type Boolean) (SweepResult :type "HitResult Structure (by ref)"))
  (bind _asbase_bpcombat (cast `/Game/Characters/BaseBPCombat` OtherActor))
  (`KismetArrayLibrary.Array_Add` (`self.BuffAffectedChars`) _asbase_bpcombat)
  (`/Game/Systems/Buffs/00_BP_AC_BuffSystem.AddBuff` (`/Game/Characters/BaseBPCombat.00_BP_AC_BuffSystem` _asbase_bpcombat) "/Game/Mods/Profession_and_Mastery/Assets/Weapons/BP_AC_Buff_Witchfire.BP_AC_Buff_Witchfire_C" self 0 (`/Game/Characters/FuncomFunctionLibrary.GetControllerFromActor` (`self.Instigator`))))

(event `self.Sphere.OnComponentEndOverlap`
  (params (OverlappedComponent :type "PrimitiveComponent Object Reference") (OtherActor :type "Actor Object Reference") (OtherComp :type "PrimitiveComponent Object Reference") (OtherBodyIndex :type Integer))
  (bind _asbase_bpcombat (cast `/Game/Characters/BaseBPCombat` OtherActor))
  (`KismetArrayLibrary.Array_RemoveItem` (`self.BuffAffectedChars`) _asbase_bpcombat))

(fn `UserConstructionScript`
  (`parent.UserConstructionScript`)
  (set `self.DamageRadius` (`SphereComponent.SphereRadius` (`self.Sphere`))))