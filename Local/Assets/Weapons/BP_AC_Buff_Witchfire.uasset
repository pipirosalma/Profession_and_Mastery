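; BP_AC_Buff_Witchfire is a buff component for the Witchfire effect, dealing periodic health damage to its owning character.
; Each tick sets the character's cause of death and applies damage scaled by stack size raised to an exponent, credited to the instigator's pawn.
; On buff start it attaches a Witchfire particle emitter to the skeletal mesh, and destroys it when the buff clears.
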(event `self.GameplayEffectToApplyOnBuffTick`
  (bind _instigator (`self.Instigator`))
  (bind _asbase_bpcombat (cast `/Game/Characters/BaseBPCombat` (`self.OwningCharacter`)))
  (set `/Game/Characters/BaseBPChar.CauseOfDeath` "NewEnumerator4" _asbase_bpcombat)
  (`GameplayStatics.ApplyDamage` (`self.GetOwner`) (* (`self.DamagePerBuffTick`) (`KismetMathLibrary.MultiplyMultiply_FloatFloat` (`KismetMathLibrary.Conv_IntToDouble` (`self.StackSize`)) (`self.DamageStackExp`))) _instigator (`Controller.K2_GetPawn` _instigator) "/Game/Systems/Progression/DmgTypeHealth_BP.DmgTypeHealth_BP_C"))

(event `self.VisualEffectToApplyOnBuffStart`
  (bind _returnvalue (`GameplayStatics.SpawnEmitterAttached` "/Game/Mods/Profession_and_Mastery/Assets/Weapons/P_Witchfire_orb_ground_collision_spawn.P_Witchfire_orb_ground_collision_spawn" (`Actor.GetComponentByClass` (`self.OwningCharacter`) "/Script/Engine.SkeletalMeshComponent")))
  (`parent.VisualEffectToApplyOnBuffStart`))

(event `self.VisualEffectToApplyOnBuffCleared`
  (`self.K2_DestroyComponent` (stale `self.VisualEffectToApplyOnBuffStart` _returnvalue))
  (`parent.VisualEffectToApplyOnBuffCleared`))