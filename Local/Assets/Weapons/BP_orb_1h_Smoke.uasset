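; Smoke variant of a one-handed orb weapon that orients its Gas component to the local player character's facing.
; On BeginPlay, outside dedicated servers, it gives Gas absolute rotation and plays the Update_liquid timeline.
; Each timeline update sets the Gas world rotation from the forward vector of player character 0, if valid.
; The parent BeginPlay runs afterwards on all instances, including dedicated servers.
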(event `self.ReceiveBeginPlay`
  (bind _returnvalue (`GameplayStatics.GetPlayerCharacter` 0))
  (`|ExecutionSequence`
    (:`then_0`
      (if (not (`KismetSystemLibrary.IsDedicatedServer`))
        (set `SceneComponent.bAbsoluteRotation` true (`self.gas`))
        (`Timeline|update_liquid`
          (:`Update`
            (`/Engine/EditorBlueprintResources/StandardMacros.IsValid` _returnvalue
              (:`Is Valid`
                (`SceneComponent.K2_SetWorldRotation` (`self.gas`) (`KismetMathLibrary.MakeRotFromX` (`self.GetActorForwardVector` _returnvalue)) false false)))))))
    (:`then_1`
      (`parent.ReceiveBeginPlay`))))

(fn `UserConstructionScript`
  (`parent.UserConstructionScript`))