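; Placeable sculpting block that lets a player of the required class carve a marble statue of the character standing under its spotlight.
; Activation sphere-traces below the light, copies the model's layout and emote, then shatters the destructible block.
; The statue gets the gender-matched emote montage frozen at its midpoint, cloth simulation disabled and marble material applied.
; Carving marks persistence dirty, and BeginPlay rebuilds already carved statues.
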(event `self.OnPlaced`
  (params (PlacedBy :type "ConanCharacter Object Reference"))
  (`SceneComponent.SetVisibility` (`self.StaticMesh`) false false))

(event `self.ReceiveBeginPlay`
  (`SceneComponent.SetVisibility` (`self.StaticMesh1`) false false)
  (`PrimitiveComponent.SetMaterial` (`self.Destructible`) 0 (`self.MarbleMaterial`))
  (if (`self.Carved`)
    (`SceneComponent.SetVisibility` (`self.SpotLight`) false false)
    (`CharacterCustomizationComponent.SetMasterSkeletalMeshComponent` (`self.BP_CharacterCustomizationComponent`) (`self.SkeletalMesh`) true)
    (`SceneComponent.SetVisibility` (`self.Destructible`) false false)
    (`self.SetUpStatue`)
    (`SceneComponent.SetVisibility` (`self.StaticMesh`) false false))
  (`parent.ReceiveBeginPlay`))

(event `SetUpStatue`
  (bind _destructible (`self.Destructible`))
  (`self.SetMontageToPlay` :!label _label
    (:`Completed`
      (`SceneComponent.SetVisibility` (`self.StaticMesh`) false false)
      (`SceneComponent.SetVisibility` (`self.StaticMesh1`) false false)
      (`SceneComponent.SetVisibility` (`self.SpotLight`) false false)
      (`CharacterCustomizationComponent.SetMasterSkeletalMeshComponent` (`self.BP_CharacterCustomizationComponent`) (`self.SkeletalMesh`) true)
      (`DestructibleComponent.ApplyRadiusDamage` _destructible 1000.0 (`SceneComponent.K2_GetComponentLocation` _destructible) 10.0 10.0 true)
      (`CharacterCustomizationComponent.SetCharacterLayout` (`self.BP_CharacterCustomizationComponent`) (`self.CharacterLayout`) false false)
      (`KismetSystemLibrary.Delay` 0.2)
      (`self.Material and Pose`)
      (`KismetSystemLibrary.Delay` 5.0)
      (`self.Material and Pose`)
      (`SceneComponent.SetVisibility` (`self.Destructible`) false false)
      (`PersistenceComponent.SetDirty` (`self.ConanBuildingPersistence`) true 5.0))))

(event `InteractableInterface.InteractableActivate`
  (params (Component :type "PrimitiveComponent Object Reference") (Instigator :type "PlayerController Object Reference") (HitIndex :type Integer))
  (bind _actormodel (`self.ActorModel`))
  (if (`self.Carved`)
    (goto _label)
    (else
      (bind _asbase_player_char (cast `/Game/Characters/BasePlayerChar` (`Controller.K2_GetPawn` Instigator)))
      (if (`|EnumEquality` (`/Game/Mods/Profession_and_Mastery/AC_Actor_Component_Main.PlayerClass` (`self.GetComponentByClass` _asbase_player_char "/Game/Mods/Profession_and_Mastery/AC_Actor_Component_Main.AC_Actor_Component_Main_C")) "NewEnumerator5")
        (set `self.Artisan` _asbase_player_char)
        (`self.TraceCast`)
        (`/Engine/EditorBlueprintResources/StandardMacros.IsValid` (`self.ActorModel`)
          (:`Is Valid`
            (bind _newparam (`/Game/Characters/BaseBPCombat.GetCurrentEmote` _actormodel))
            (set `self.EmoteToTake` _newparam)
            (bind _character_layout (`/Game/Characters/BasePlayerChar.GetCharacterLayout` _actormodel))
            (bind _output_get (set `self.CharacterLayout` _character_layout))
            (`self.GenderCheck` _output_get)
            (set `self.Carved` true)
            (`/Game/Mods/Profession_and_Mastery/AC_Actor_Component_Main.EffectsToPlay` (`self.GetComponentByClass` (`self.Artisan`) "/Game/Mods/Profession_and_Mastery/AC_Actor_Component_Main.AC_Actor_Component_Main_C") "/Game/Characters/humans/animations/combat/1h_pickaxe/AM_combat_1h_pickaxe_3rd.AM_combat_1h_pickaxe_3rd" true 0 null (0.0 0.0 0.0) null)
            (`self.SetUpStatue`))
          (:`Is Not Valid`
            (set `self.ErrorMessage` "You find no model under the spotlight")
            (`self.Notification` :!label _label_2)))
        (else
          (set `self.ErrorMessage` "You don't know how to carve this material ")
          (goto _label_2))))))

(event `Notification`
  (message `/Game/Characters/HUDNotification_Interface.NotificationText` (stale `InteractableInterface.InteractableActivate` Instigator) (`self.ErrorMessage`) false))

(event `TraceCast`
  (bind _returnvalue (`SceneComponent.K2_GetComponentLocation` (`self.SpotLight`)))
  (bind _outhits (`KismetSystemLibrary.SphereTraceMulti` :`Start` _returnvalue :`End` (+ _returnvalue (0.0 0.0 -500.0)) :`Radius` 20.0 :`TraceChannel` "TraceTypeQuery1" :`DrawDebugType` "ForDuration" :`bIgnoreSelf` false))
  (for _array_element _outhits
    (bind _asbase_player_char (cast `/Game/Characters/BasePlayerChar` (`.HitActor` (`GameplayStatics.BreakHitResult` _array_element))))
    (set `self.ActorModel` _asbase_player_char)))

(fn `PlayAnimationFromEmote`
  (params (Target :type "SkeletalMeshComponent Object Reference"))
  (bind _animmonatgetoplay (`self.AnimMonatgeToPlay`))
  (bind _object (`|ConvertAsset` _animmonatgetoplay))
  (`/Engine/EditorBlueprintResources/StandardMacros.IsAssetValid` _animmonatgetoplay
    (:`IsValid`
      (`SkeletalMeshComponent.PlayAnimation` Target _object false)
      (bind _returnvalue (`AnimSequenceBase.GetPlayLength` _object))
      (`SkeletalMeshComponent.SetPosition` Target (/ _returnvalue 2.0) false))
    (:`Is Not Valid`
      _))
  (`SkeletalMeshComponent.SetPlayRate` Target 0.0))

(fn `UserConstructionScript`
  (`parent.UserConstructionScript`))