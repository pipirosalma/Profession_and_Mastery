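; BP_PL_CraftingStation_Easel is a placeable crafting station whose mesh reflects what its inventory holds.
; When items are added to or removed from the placeable inventory, it checks for one item of a specific template ID and swaps the static mesh between dryer on and off variants.
; The construction script defers to the parent, and the artisan thrall inventory getter is an empty override.
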(event `self.PlaceableInventory.SignalItemAdded`
  (params (index :type Integer) (item :type "GameItem Object Reference") (srcInventory :type "ItemInventory Object Reference") (srcIndex :type Integer))
  (if (`ItemInventory.HasItemByTemplateID` (`self.PlaceableInventory`) 80311 1) :!label _label
    (`StaticMeshComponent.SetStaticMesh` (`self.StaticMesh`) "/Game/Environment/Player_built/Meshes/SM_dryer_on.SM_dryer_on")
    (else
      (`StaticMeshComponent.SetStaticMesh` (`self.StaticMesh`) "/Game/Environment/Player_built/Meshes/SM_dryer_off.SM_dryer_off"))))

(event `self.PlaceableInventory.SignalItemRemoved`
  (params (index :type Integer) (item :type "GameItem Object Reference") (dstInventory :type "ItemInventory Object Reference") (dstIndex :type Integer))
  (goto _label))

(fn `GetArtisanThrallInventory`
  (returns (ReturnValue :type "ItemInventory Object Reference"))
  (return null))

(fn `UserConstructionScript`
  (`parent.UserConstructionScript`))