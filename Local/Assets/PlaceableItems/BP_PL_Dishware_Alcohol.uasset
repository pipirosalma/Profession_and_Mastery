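; Placeable alcohol jug that players interact with to drink, using charge and status logic inherited from a well-style parent.
; When empty, it consumes five wine items from the player to refill its charges, or shows a warning if the backpack lacks them.
; Otherwise, players with a hunger component gain the drunkenness buff and hydration, a charge is spent, and a drink montage plays.
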(event `/Game/Systems/Building/Placeables/BP_Master_Placeables.InteractableActivate`
  (params (Component :type "PrimitiveComponent Object Reference") (Instigator :type "PlayerController Object Reference") (HitIndex :type Integer))
  (bind _returnvalue (`Controller.K2_GetPawn` Instigator))
  (bind _returnvalue_2 (`self.K2_GetComponentsByClass` _returnvalue "/Game/Systems/Hunger/BP_HungerSystem.BP_HungerSystem_C"))
  (if (== (`self.CurDrinkCharges`) 0.0)
    (bind _asconan_character (cast `ConanCharacter` _returnvalue))
    (bind _returnvalue_3 (`ConanCharacter.GetBackpackInventory` _asconan_character))
    (if (`ItemInventory.HasItemByTemplateID` _returnvalue_3 18078 5)
      (bind _success (`/Game/Systems/MiscFunctions.DeleteItemsInAllInventoriesByTemplateID` Instigator 18078 5))
      (if _success
        (set `self.CurDrinkCharges` 30.0))
      (else
        (bind _asfun_combat_player_controller (cast `/Game/Systems/FunCombat_PlayerController` Instigator))
        (`/Game/Systems/FunCombat_PlayerController.NotificationText` _asfun_combat_player_controller "The jug is empty! ((need 5 glass of wine))" false)))
    (else
      (bind _asbase_player_char (cast `/Game/Characters/BasePlayerChar` _returnvalue))
      (if (> (`KismetArrayLibrary.Array_Length` _returnvalue_2) 0)
        (`/Game/Systems/Buffs/00_BP_AC_BuffSystem.AddBuff` (`/Game/Characters/BaseBPCombat.00_BP_AC_BuffSystem` _asbase_player_char) "/Game/Systems/Buffs/Alcohol/BP_AC_Buff_Drunkenness.BP_AC_Buff_Drunkenness_C" Instigator 0 Instigator)
        (`/Game/Systems/Hunger/BP_HungerSystem.ServerDrink` (`KismetArrayLibrary.Array_Get` _returnvalue_2) (`self.OnInteractDrinkValue`))
        (`self.DecrementDrinkCharges`)
        (`self.ForceUpdateWellStatus`)
        (bind _asbase_player_char_2 (cast `/Game/Characters/BasePlayerChar` _returnvalue))
        (`self.AnimToPlay` _asbase_player_char_2)))))

(event `AnimToPlay`
  (params (BasePlayerChar :type "/Game/Characters/BasePlayerChar Object Reference"))
  (`Character.PlayAnimMontage` BasePlayerChar "/Game/Mods/Profession_and_Mastery/Assets/Animation/AM_Drink_F.AM_Drink_F" 1.0 "None"))

(fn `UserConstructionScript`
  (`parent.UserConstructionScript`))