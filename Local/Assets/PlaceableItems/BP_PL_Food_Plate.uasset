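; Placeable plate item (named Food Plate) that displays the item in its first inventory slot as a mesh, though it only accepts shield-archetype items for display.
; On begin play it caches the slot transform, clears the mesh and attaches a client inventory monitor.
; Inventory add, remove and stat-change signals rebuild the display: reset the slot, async-load the item's visual mesh, then apply a weapon-type location and rotation offset.
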(event `self.ReceiveBeginPlay`
  (bind _slot0 (`self.Slot0`))
  (set `self.Initial Location Slot 0` (`SceneComponent.K2_GetComponentLocation` _slot0))
  (set `self.Initial Rotation Slot 0` (`SceneComponent.K2_GetComponentRotation` _slot0))
  (bind _returnvalue (`|GenericCreateObject` "/Script/ConanSandbox.ItemInventoryClientMonitor" self))
  (bind _output_get (set `self.ShieldInventoryMonitor` _returnvalue))
  (`ItemInventoryClientMonitor.SetInventory` _output_get (`self.PlaceableInventory`))
  (`StaticMeshComponent.SetStaticMesh` (`self.Slot0`) null)
  (`parent.ReceiveBeginPlay`))

(event `self.PlaceableInventory.SignalItemRemoved`
  (params (index :type Integer) (item :type "GameItem Object Reference") (dstInventory :type "ItemInventory Object Reference") (dstIndex :type Integer))
  (bind _slot0 (`self.Slot0`))
  (`StaticMeshComponent.SetStaticMesh` (`self.Slot0`) (`self.EmptyMesh`) :!label _label)
  (if (`KismetSystemLibrary.IsValid` (`ItemInventory.GetItem` (`self.PlaceableInventory`) 0))
    (`self.CheckForValidItems` 0)
    (if (`self.ValidItem`)
      (`SceneComponent.K2_SetWorldLocationAndRotation` _slot0 (`self.Initial Location Slot 0`) (`self.Initial Rotation Slot 0`) false false)
      (`SceneComponent.ResetRelativeTransform` _slot0)
      (bind _object (`|LoadAsset` (`GameItem.VisualStaticMesh` (`ItemInventory.GetItem` (`self.PlaceableInventory`) 0))))
      (`StaticMeshComponent.SetStaticMesh` (`self.Slot0`) _object)
      (`self.ModifyLocationRotation` 0)
      (`SceneComponent.K2_AddRelativeLocation` (`self.Slot0`) (`self.LocationMod`) false false)
      (`SceneComponent.K2_AddRelativeRotation` (`self.Slot0`) (`self.RotationMod`) false false))))

(event `self.PlaceableInventory.SignalItemAdded`
  (params (index :type Integer) (item :type "GameItem Object Reference") (srcInventory :type "ItemInventory Object Reference") (srcIndex :type Integer))
  (goto _label))

(event `self.PlaceableInventory.SignalItemFloatStatChanged`
  (params (item :type "GameItem Object Reference") (statID :type "EItemFloatStatID Enum" :default "WeaponStaminaHeavyChargedRegenModifier") (statValue :type "Float (single-precision)") (deltaValue :type "Float (single-precision)"))
  (goto _label))

(event `self.PlaceableInventory.SignalItemIntStatChanged`
  (params (item :type "GameItem Object Reference") (statID :type "EItemIntStatID Enum" :default "MaxStackSize") (statValue :type Integer) (deltaValue :type Integer))
  (goto _label))

(fn `CheckForValidItems`
  (params (index :type Integer))
  (if (`|EnumEquality` (`GameItem.WeaponArcheType` (`ItemInventory.GetItem` (`self.PlaceableInventory`) index)) "Shield")
    (set `self.ValidItem` true)
    (else
      (set `self.ValidItem` false))))

(fn `ModifyLocationRotation`
  (params (index :type Integer))
  (switch `WeaponItemTypes` (cast `WeaponItemTypes` (`KismetMathLibrary.Conv_IntToByte` (`GameItem.GetIntStat` (`ItemInventory.GetItem` (`self.PlaceableInventory`) index) "WeaponType")))
    (:`Shield`
      (set `self.RotationMod` (struct :`Roll` 270.0))
      (set `self.LocationMod` (30.0 5.0 0.0)))))

(fn `UserConstructionScript`
  (`parent.UserConstructionScript`))