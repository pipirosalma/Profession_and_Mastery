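; Poisoned variant of a placeable drink dishware item that lets players drink from it and poisons them.
; On interact, if charges remain, it feeds the drink value to the pawn's BP_HungerSystem, spends a charge and updates well status.
; It then calls a montage event and applies the BP_deBuff_PoisonedFood debuff through the character's buff system.
; Purified-water refill logic is present but disconnected, so it never runs.
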(event `/Game/Systems/Building/Placeables/BP_Master_Placeables.InteractableActivate`
  (params (Component :type "PrimitiveComponent Object Reference") (Instigator :type "PlayerController Object Reference") (HitIndex :type Integer))
  (bind _returnvalue (`Controller.K2_GetPawn` Instigator))
  (bind _returnvalue_2 (`self.K2_GetComponentsByClass` _returnvalue "/Game/Systems/Hunger/BP_HungerSystem.BP_HungerSystem_C"))
  (if (== (`self.CurDrinkCharges`) 0.0)
    _
    (elif (> (`KismetArrayLibrary.Array_Length` _returnvalue_2) 0)
      (`/Game/Systems/Hunger/BP_HungerSystem.ServerDrink` (`KismetArrayLibrary.Array_Get` _returnvalue_2) (`self.OnInteractDrinkValue`))
      (`self.DecrementDrinkCharges`)
      (`self.ForceUpdateWellStatus`)
      (bind _asbase_player_char (cast `/Game/Characters/BasePlayerChar` _returnvalue))
      (`self.AnimToPlay` _asbase_player_char)
      (`/Game/Systems/Buffs/00_BP_AC_BuffSystem.AddBuff` (`/Game/Characters/BaseBPCombat.00_BP_AC_BuffSystem` _asbase_player_char) "/Game/Mods/Profession_and_Mastery/System/Buffs/BP_deBuff_PoisonedFood.BP_deBuff_PoisonedFood_C" null 0 null))))

(event `AnimToPlay`
  (params (BasePlayerChar :type "/Game/Characters/BasePlayerChar Object Reference"))
  (`Character.PlayAnimMontage` BasePlayerChar null 1.0 "None"))

(fn `UserConstructionScript`
  (`parent.UserConstructionScript`))