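; Placeable sculptor item that, on client interaction, copies the interacting player's character onto its skeletal mesh as a gold statue.
; It adds a character customization component built from the player's layout, with SkeletalMesh as master.
; Gold statue material instances are created on the third primitive component's first slot and replace the component's dynamic material list.
; Stone material, frozen pose and mesh override experiments remain unconnected.
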(event `InteractableInterface.ClientInteractableActivate`
  (params (Component :type "PrimitiveComponent Object Reference") (Instigator :type "PlayerController Object Reference") (HitIndex :type Integer))
  (bind _newvar_1 (`self.NewVar_1`))
  (bind _asbase_player_char (cast `/Game/Characters/BasePlayerChar` (`Controller.K2_GetPawn` Instigator)))
  (bind _character_layout (`/Game/Characters/BasePlayerChar.GetCharacterLayout` _asbase_player_char))
  (bind _returnvalue (`AddComponent|NODE_AddBP_CharacterCustomizationComponent-2` :`Layout` _character_layout :`Master` (`self.SkeletalMesh`)))
  (bind _matparamcontroller (message `/Game/Systems/Interfaces/IsCorpseInterface.GetDynamicMaterialParamController` _returnvalue))
  (for _ (`/Game/Effects/blueprints/DynamicMaterialParamController.DynamicMaterialInstances` _matparamcontroller)
    (bind _returnvalue_2 (`PrimitiveComponent.CreateDynamicMaterialInstance` (`KismetArrayLibrary.Array_Get` (`self.K2_GetComponentsByClass` (`ActorComponent.GetOwner` _returnvalue) "/Script/Engine.PrimitiveComponent") 2) 0 "/Game/Environment/Player_built/Materials/Ml_avatar_mitra_statue_gold.Ml_avatar_mitra_statue_gold"))
    (`KismetArrayLibrary.Array_Add` _newvar_1 _returnvalue_2))
  (set `/Game/Effects/blueprints/DynamicMaterialParamController.DynamicMaterialInstances` _newvar_1 _matparamcontroller))

(fn `UserConstructionScript`
  (`parent.UserConstructionScript`))