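; Actor component on the player character that fills a serving object with a consumable from the backpack.
; A request passes through SRV and C events, then removes one item and copies its ID, food and drink amounts from ItemTable.
; It constructs the item class to read its buffs: food merges its own with the serving's, alcohol adds Drunkenness, and poison adds its buff.
; Food and poison make the serving mesh visible; the Spice input is unused.
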(event `ServingConsumable`
  (params (ServingPL :type "/Game/Mods/Profession_and_Mastery/System/BP_FoodPlate_Master Object Reference") (ConsumableID :type Integer) (Spice :type Boolean))
  (`self.ServingConsumable_SRV` ServingPL ConsumableID Spice))

(event `ServingConsumable_SRV`
  (params (ServingPL :type "/Game/Mods/Profession_and_Mastery/System/BP_FoodPlate_Master Object Reference") (ConsumableID :type Integer) (Spice :type Boolean))
  (`self.ServingConsumable_C` ServingPL ConsumableID Spice))

(event `ServingConsumable_C`
  (params (ServingPL :type "/Game/Mods/Profession_and_Mastery/System/BP_FoodPlate_Master Object Reference") (ConsumableID :type Integer) (Spice :type Boolean))
  (bind _mergedbuff (`self.MergedBuff`))
  (bind _asbase_player_char (cast `/Game/Characters/BasePlayerChar` (`self.GetOwner`)))
  (`ItemInventory.ValidatedDeleteItemsByTemplate` (`/Game/Characters/BasePlayerChar.BackpackInventory` _asbase_player_char) ConsumableID 1)
  (set `/Game/Mods/Profession_and_Mastery/System/BP_FoodPlate_Master.TemplateItemID` ConsumableID ServingPL)
  (bind _returnvalue (`|GetDataTableRow` "/Game/Items/ItemTable.ItemTable" (`KismetStringLibrary.Conv_StringToName` (`KismetStringLibrary.Conv_IntToString` ConsumableID)))
    (:`then`
      (bind ((`Name` _name) (`Icon` _icon) (`ItemClass` _itemclass) (`GUICategory` _guicategory) (`FoodAmount` _foodamount) (`DrinkAmount` _drinkamount)) (break `ItemTableRow` _returnvalue))
      (set `/Game/Mods/Profession_and_Mastery/System/BP_FoodPlate_Master.FoodAmount` _foodamount ServingPL)
      (set `/Game/Mods/Profession_and_Mastery/System/BP_FoodPlate_Master.DrinkAmount` _drinkamount ServingPL)
      (set `/Game/Mods/Profession_and_Mastery/System/BP_FoodPlate_Master.IsEmpty` false ServingPL)
      (bind _returnvalue_2 (`|GenericCreateObject` (`|ConvertAsset` _itemclass) ServingPL))
      (bind _asbpgame_item_food (cast `/Game/Items/Hunger/BPGameItemFood` _returnvalue_2)
        (:`then`
          (cast `/Game/Items/Hunger/BPGameItemFood_Master_Alcohol` _asbpgame_item_food
            (:`then`
              (`KismetArrayLibrary.Array_Add` (`self.MergedBuff`) "/Game/Systems/Buffs/Alcohol/BP_AC_Buff_Drunkenness.BP_AC_Buff_Drunkenness_C"))
            (:`CastFailed`
              _))
          (`KismetArrayLibrary.Array_Append` _mergedbuff (`/Game/Items/Hunger/BPGameItemFood.Buffs On Use` _asbpgame_item_food))
          (`KismetArrayLibrary.Array_Append` _mergedbuff (`/Game/Mods/Profession_and_Mastery/System/BP_FoodPlate_Master.BuffsOnUse` ServingPL)))
        (:`CastFailed`
          (bind _asbp_game_item_base_poison (cast `/Game/Items/Poisons/BP_GameItem_BasePoison` _returnvalue_2))
          (`KismetArrayLibrary.Array_Add` (`self.MergedBuff`) (`/Game/Items/Poisons/BP_GameItem_BasePoison.BuffClass` _asbp_game_item_base_poison))))
      (set `/Game/Mods/Profession_and_Mastery/System/BP_FoodPlate_Master.BuffsOnUse` (`self.MergedBuff`) ServingPL)
      (`SceneComponent.SetVisibility` (`/Game/Mods/Profession_and_Mastery/System/BP_FoodPlate_Master.StaticMesh1` ServingPL) true false))))