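; Player spell-casting component for a Conan Exiles mod, handling channeled god spells and a Ymir hammer cast, both adding corruption.
; While corruption permits, Tick runs Cobra Dance, debuffing nearby pawns not worshipping the spell's god, with corruption-derived potency.
; Leaving the channel spot ends it and removes the debuff from that area.
; YmirHammer briefly equips a spawned maul for montage and snow effects; timer-based channeling is unused.
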(event `InitializeChannelDebuff`
  (params (ChannelingInProgress :type Integer) (SpellGod :type String) (SpellBuffToAdd :type "/Game/Systems/Buffs/01_BP_AC_Buff_Master Class Reference") (SpellAnimMontage :type "AnimMontage Object Reference"))
  (bind _asbase_player_char (`self.GetBasePlayer`))
  (set `self.ChannelingInProgress` ChannelingInProgress)
  (set `self.ChannelingLocation` (`Actor.K2_GetActorLocation` _asbase_player_char))
  (set `self.SpellGod` SpellGod)
  (set `self.SpellBuffToAdd` SpellBuffToAdd)
  (bind _output_get (set `self.SpellAnimMontage` SpellAnimMontage))
  (`/Game/Mods/Profession_and_Mastery/AC_Actor_Component_Main.EffectsToPlay` (`Actor.GetComponentByClass` _asbase_player_char "/Game/Mods/Profession_and_Mastery/AC_Actor_Component_Main.AC_Actor_Component_Main_C") _output_get true 0 null (0.0 0.0 0.0) null))

(event `self.ReceiveTick`
  (params (DeltaSeconds :type "Float (single-precision)"))
  (bind (_value _returnvalue) (`BlueprintMapLibrary.Map_Find` (`self.ChanneledSpells`) (`self.ChannelingInProgress`)))
  (if _returnvalue
    (if (<= (`EnergyReceiverComponent.GetEnergy` (`/Game/Characters/BasePlayerChar.BPEnergyReceiver` (`self.GetBasePlayer`)) "EnergyType_Corruption") 1800.0)
      (switch `name` _value
        (:`CobraDance`
          (`self.SnakeDance`))))))

(event `SnakeDanceChannel`
  ;[1 1 1] unused
  (switch `name` (`BlueprintMapLibrary.Map_Find` (`self.ChanneledSpells`) (`self.ChannelingInProgress`))
    (:`CobraDance`
      (`self.SnakeDance`)
      (add `Character.OnCharacterMovementUpdated` (`self.GetBasePlayer`) (delegate `Interruption`)))))

(event `Interruption`
  (params (DeltaSeconds :type "Float (double-precision)") (OldLocation :type "Vector Structure") (OldVelocity :type "Vector Structure"))
  ;[1 1 1] unused
  (if (not (== (- (`Actor.GetVelocity` (`self.GetBasePlayer`)) OldVelocity) (0.0 0.0 0.0)))
    (`KismetSystemLibrary.K2_ClearAndInvalidateTimerHandle` (`self.CastingLoopTimer`))))

(event `YmirHammer`
  (bind _asbase_player_char (`self.GetBasePlayer`))
  (bind _returnvalue (`Actor.GetComponentByClass` _asbase_player_char "/Game/Mods/Profession_and_Mastery/AC_Actor_Component_Main.AC_Actor_Component_Main_C"))
  (bind _bpenergyreceiver (`/Game/Characters/BasePlayerChar.BPEnergyReceiver` (`self.GetBasePlayer`)))
  (bind _equipmentinventory (`/Game/Characters/BaseBPChar.EquipmentInventory` _asbase_player_char))
  (`EquipmentInventory.UnequipAllWeapons` _equipmentinventory)
  (bind _returnvalue_2 (`GameItemSpawner.SpawnItem` "GameItem" 8941086))
  (`EquipmentInventory.AddItemToSlot` _equipmentinventory "MainHand" _returnvalue_2)
  (`/Game/Mods/Profession_and_Mastery/AC_Actor_Component_Main.EffectsToPlay` _returnvalue "/Game/Mods/Profession_and_Mastery/Assets/Animation/AM_combat_Ymir_Maul.AM_combat_Ymir_Maul" true 0 null (0.0 0.0 0.0) null)
  (`KismetSystemLibrary.Delay` 1.0)
  (`/Game/Mods/Profession_and_Mastery/AC_Actor_Component_Main.EffectsToPlay` _returnvalue "/Game/Mods/Profession_and_Mastery/Assets/Animation/AM_combat_Ymir_Maul.AM_combat_Ymir_Maul" true 1 "/Game/weathereffects/Particles/NewParticles/P_Snow_Swirl.P_Snow_Swirl" (`Actor.K2_GetActorLocation` _asbase_player_char) "/Game/Mods/Profession_and_Mastery/System/Spells/BP_Spell_ParticleEmiter.BP_Spell_ParticleEmiter_C")
  (if (not (>= (`EnergyReceiverComponent.GetEnergy` _bpenergyreceiver "EnergyType_Corruption") 1700.0))
    (`EnergyReceiverComponent.ModifyEnergy` _bpenergyreceiver "EnergyType_Corruption" 200.0))
  (`EquipmentInventory.UnequipAllWeapons` (`/Game/Characters/BaseBPChar.EquipmentInventory` (`self.GetBasePlayer`)))
  (`self.RemoveAllItems` 8941086))

(fn `GetBasePlayer`
  (returns (`AsBase Player Char` :type "/Game/Characters/BasePlayerChar Object Reference"))
  (bind _asbase_player_char (cast `/Game/Characters/BasePlayerChar` (`self.GetOwner`))
    (:`then`
      _)
    (:`CastFailed`
      _))
  (return _asbase_player_char))

(fn `RemoveAllItems`
  (params (ItemId :type Integer))
  (locals (InventoryTypes :type "Array of EInventoryType Enum"))
  (for _array_element (`local.InventoryTypes`)
    (bind _returnvalue (`ItemInventory.GetInventoryByType` (`self.GetBasePlayer`) _array_element))
    (`ItemInventory.ValidatedDeleteItemsByTemplate` _returnvalue ItemId (`ItemInventory.GetNumberOfItemsByTemplate` _returnvalue ItemId))))

(fn `SnakeDance`
  (bind _returnvalue (`self.GetOwner`))
  (bind _controller (`/Game/Characters/FuncomFunctionLibrary.GetControllerFromActor` _returnvalue))
  (bind _returnvalue_2 (`EnergyReceiverComponent.ModifyEnergy` (`/Game/Characters/BasePlayerChar.BPEnergyReceiver` (`self.GetBasePlayer`)) "EnergyType_Corruption" 5.0))
  (set `self.BuffPotency` (`KismetMathLibrary.FTrunc` (/ _returnvalue_2 100.0)))
  (bind _outactors (`GameplayStatics.GetAllActorsOfClass` "/Script/ConanSandbox.ConanWorldSettings"))
  (bind _returnvalue_3 (`ConanWorldSettings.GetPlayerPawnRegistry` (`KismetArrayLibrary.Array_Get` _outactors)))
  (bind _returnvalue_4 (`PlayerPawnRegistry.GetPawnsWithinDistance` _returnvalue_3 (`self.ChannelingLocation`) 1000.0))
  (for _array_element _returnvalue_4
    (bind _returnvalue_5 (`Actor.K2_GetComponentsByClass` _array_element "/Game/Systems/Buffs/00_BP_AC_BuffSystem.00_BP_AC_BuffSystem_C"))
    (if (> (`KismetArrayLibrary.Array_Length` _returnvalue_5) 0)
      (bind _item (`KismetArrayLibrary.Array_Get` _returnvalue_5))
      (`self.GodPresenceCheck` (`self.SpellGod`) _item
        (:`false`
          (`/Game/Systems/Buffs/00_BP_AC_BuffSystem.AddBuff` _item (`self.SpellBuffToAdd`) _controller (`self.BuffPotency`) _controller)))))
  (if (not (== (- (`Actor.K2_GetActorLocation` _returnvalue) (`self.ChannelingLocation`)) (0.0 0.0 0.0) :`ErrorTolerance` 100.0))
    (set `self.ChannelingInProgress` 0)
    (`/Game/Mods/Profession_and_Mastery/AC_Actor_Component_Main.EffectsToPlay` (`Actor.GetComponentByClass` (`self.GetBasePlayer`) "/Game/Mods/Profession_and_Mastery/AC_Actor_Component_Main.AC_Actor_Component_Main_C") (`self.SpellAnimMontage`) false 0 null (0.0 0.0 0.0) null)
    (bind _outactors_2 (`GameplayStatics.GetAllActorsOfClass` "/Script/ConanSandbox.ConanWorldSettings"))
    (bind _returnvalue_6 (`ConanWorldSettings.GetPlayerPawnRegistry` (`KismetArrayLibrary.Array_Get` _outactors_2)))
    (bind _returnvalue_7 (`PlayerPawnRegistry.GetPawnsWithinDistance` _returnvalue_6 (`self.ChannelingLocation`) 1000.0))
    (for _array_element_2 _returnvalue_7
      (bind _returnvalue_8 (`Actor.K2_GetComponentsByClass` _array_element_2 "/Game/Systems/Buffs/00_BP_AC_BuffSystem.00_BP_AC_BuffSystem_C"))
      (if (> (`KismetArrayLibrary.Array_Length` _returnvalue_8) 0)
        (`/Game/Systems/Buffs/00_BP_AC_BuffSystem.RemoveBuff` (`KismetArrayLibrary.Array_Get` _returnvalue_8) (`self.SpellBuffToAdd`))))))